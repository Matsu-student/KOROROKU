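; BP_OutGamePC is the out-game player controller that routes menu navigation input to a target widget.
; Enhanced Input actions for decide, cancel, up, down, left and right each call the matching message function on TatgetWidget, passing the action value.
; The controller holds no UI logic of its own and leaves the response to that widget.
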(event `EnhancedInput|/Game/Game/Input/Key/IA_KeyDecide`
  (params (ActionValue :type Boolean) (ElapsedSeconds :type "Float (double-precision)") (TriggeredSeconds :type "Float (double-precision)") (InputAction :type "InputAction Object Reference" :default "/Game/Game/Input/Key/IA_KeyDecide.IA_KeyDecide"))
  (:`Triggered`
    (message `/Game/Game/OutGame/PlayerController/BI_OutGamePC.Decide` (`self.TatgetWidget`) ActionValue)))

(event `EnhancedInput|/Game/Game/Input/Key/IA_KeyCancel`
  (params (ActionValue :type Boolean) (ElapsedSeconds :type "Float (double-precision)") (TriggeredSeconds :type "Float (double-precision)") (InputAction :type "InputAction Object Reference" :default "/Game/Game/Input/Key/IA_KeyCancel.IA_KeyCancel"))
  (:`Triggered`
    (message `/Game/Game/OutGame/PlayerController/BI_OutGamePC.Cancel` (`self.TatgetWidget`) ActionValue)))

(event `EnhancedInput|/Game/Game/Input/Key/IA_KeyUP`
  (params (ActionValue :type Boolean) (ElapsedSeconds :type "Float (double-precision)") (TriggeredSeconds :type "Float (double-precision)") (InputAction :type "InputAction Object Reference" :default "/Game/Game/Input/Key/IA_KeyUP.IA_KeyUP"))
  (:`Triggered`
    (message `/Game/Game/OutGame/PlayerController/BI_OutGamePC.UP` (`self.TatgetWidget`) ActionValue)))

(event `EnhancedInput|/Game/Game/Input/Key/IA_KeyDawn`
  (params (ActionValue :type Boolean) (ElapsedSeconds :type "Float (double-precision)") (TriggeredSeconds :type "Float (double-precision)") (InputAction :type "InputAction Object Reference" :default "/Game/Game/Input/Key/IA_KeyDawn.IA_KeyDawn"))
  (:`Triggered`
    (message `/Game/Game/OutGame/PlayerController/BI_OutGamePC.Dawn` (`self.TatgetWidget`) ActionValue)))

(event `EnhancedInput|/Game/Game/Input/Key/IA_KeyLeft`
  (params (ActionValue :type Boolean) (ElapsedSeconds :type "Float (double-precision)") (TriggeredSeconds :type "Float (double-precision)") (InputAction :type "InputAction Object Reference" :default "/Game/Game/Input/Key/IA_KeyLeft.IA_KeyLeft"))
  (:`Triggered`
    (message `/Game/Game/OutGame/PlayerController/BI_OutGamePC.left` (`self.TatgetWidget`) ActionValue)))

(event `EnhancedInput|/Game/Game/Input/Key/IA_KeyRight`
  (params (ActionValue :type Boolean) (ElapsedSeconds :type "Float (double-precision)") (TriggeredSeconds :type "Float (double-precision)") (InputAction :type "InputAction Object Reference" :default "/Game/Game/Input/Key/IA_KeyRight.IA_KeyRight"))
  (:`Triggered`
    (message `/Game/Game/OutGame/PlayerController/BI_OutGamePC.Right` (`self.TatgetWidget`) ActionValue)))

(fn `UserConstructionScript`)