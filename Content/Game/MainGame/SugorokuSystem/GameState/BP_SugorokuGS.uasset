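; BP_SugorokuGS is the GameState for the Sugoroku board-game mode, coordinating startup once loading finishes.
; On BeginPlay it spawns and keeps an item storage actor and a load checker actor.
; LoadEnd runs GameInit, then destroys the load checker.
; GameInit finds and initializes every player controller, player state (passing its index), player actor and game mode, in that order.
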(event `self.ReceiveBeginPlay`
  (bind _returnvalue (`|SpawnActorFromClass` "/Game/Game/MainGame/SugorokuSystem/ItemStrage/BP_ItemStorage.BP_ItemStorage_C" (`KismetMathLibrary.MakeTransform` (0.0 0.0 0.0)) "Undefined" "MultiplyWithRoot" null null))
  (set `self.ItemStorage` _returnvalue)
  (bind _returnvalue_2 (`|SpawnActorFromClass` "/Game/Game/MainGame/SugorokuSystem/GameState/BP_SugorokuLoadChecker.BP_SugorokuLoadChecker_C" (`KismetMathLibrary.MakeTransform` (0.0 0.0 0.0)) "Undefined" "MultiplyWithRoot" null null))
  (set `self.LoadChecker` _returnvalue_2))

(event `GameInit`
  (bind _outactors (`GameplayStatics.GetAllActorsOfClass` "/Game/Game/MainGame/SugorokuSystem/PlayerController/BP_SugorokuPC.BP_SugorokuPC_C"))
  (for _array_element _outactors
    (`/Game/Game/MainGame/SugorokuSystem/PlayerController/BP_SugorokuPC.init` _array_element))
  (bind _outactors_2 (`GameplayStatics.GetAllActorsOfClass` "/Game/Game/MainGame/SugorokuSystem/PlayerState/BP_SugorokuPS.BP_SugorokuPS_C"))
  (for (_array_element_2 _array_index) _outactors_2
    (`/Game/Game/MainGame/SugorokuSystem/PlayerState/BP_SugorokuPS.init` _array_element_2 _array_index))
  (bind _outactors_3 (`GameplayStatics.GetAllActorsOfClass` "/Game/Game/MainGame/SugorokuSystem/Player/BP_SugorokuPlayer.BP_SugorokuPlayer_C"))
  (for _array_element_3 _outactors_3
    (`/Game/Game/MainGame/SugorokuSystem/Player/BP_SugorokuPlayer.Init` _array_element_3))
  (bind _outactors_4 (`GameplayStatics.GetAllActorsOfClass` "/Game/Game/MainGame/SugorokuSystem/Gamemode/BP_SugorokuGM.BP_SugorokuGM_C"))
  (for _array_element_4 _outactors_4
    (`/Game/Game/MainGame/SugorokuSystem/Gamemode/BP_SugorokuGM.Init` _array_element_4)))

(fn `LoadEnd`
  (`self.GameInit`)
  (`self.K2_DestroyActor` (`self.LoadChecker`))
  (set `self.LoadChecker` null))

(fn `UserConstructionScript`)