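; BP_TileSercher is a helper actor for the sugoroku board game that steps along linked tiles for a given move count.
; SetNowTile stores the current tile and collects it uniquely in SerchTiles.
; Each TeleportNextTile call jumps to the end of the first next tile's spline, queueing other branches of selectable tiles with their remaining moves.
; When moves run out, it resumes from the oldest queued branch; the backward path is hard-wired off.
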(event `self.ReceiveBeginPlay`)

(fn `SetNowTile`
  (params (NowTile :type "/Game/Game/MainGame/SugorokuSystem/Props/Tiles/Tile/BP_TileBase Object Reference"))
  (bind _output_get (set `self.NowTile` NowTile))
  (`KismetArrayLibrary.Array_AddUnique` (`self.SerchTiles`) _output_get))

(fn `Teleport`
  (params (Load :type "/Game/Game/MainGame/SugorokuSystem/Props/Load/BP_LoadBase Object Reference"))
  (bind _spline (`/Game/Game/MainGame/SugorokuSystem/Props/Load/BP_LoadBase.Spline` Load))
  (if (!= Load null)
    (`self.K2_SetActorLocation` (`SplineComponent.GetLocationAtDistanceAlongSpline` _spline (`SplineComponent.GetSplineLength` _spline) "World"))))

(fn `TeleportNextTile`
  (returns (SerchEnd :type Boolean))
  (locals (Load :type "/Game/Game/MainGame/SugorokuSystem/Props/Load/BP_LoadBase Object Reference"))
  (bind _nexttile (`/Game/Game/MainGame/SugorokuSystem/Props/Tiles/Tile/BP_TileBase.NextTile` (`self.NowTile`)))
  (bind (_load _movenum) (break `/Game/Game/MainGame/SugorokuSystem/Props/TileSercher/F_Destination` (`|GetArrayItem` (`self.Destinations`))))
  (bind _returnvalue (`KismetArrayLibrary.Array_Length` _nexttile))
  (if (> (`self.MoveNum`) 0)
    (if (`/Game/Game/MainGame/SugorokuSystem/Props/Tiles/Tile/BP_TileBase.CanSelect` (`self.NowTile`))
      (if (> _returnvalue 1)
        (for _index (range 1 _returnvalue)
          (`KismetArrayLibrary.Array_Add` (`self.Destinations`) (make `/Game/Game/MainGame/SugorokuSystem/Props/TileSercher/F_Destination` (`|GetArrayItem` _nexttile _index) (`self.MoveNum`))))))
    (if true
      (set `local.Load` (`|GetArrayItem` (`/Game/Game/MainGame/SugorokuSystem/Props/Tiles/Tile/BP_TileBase.NextTile` (`self.NowTile`))))
      (`/Engine/EditorBlueprintResources/StandardMacros.DecrementInt` (`self.MoveNum`)
        (:`  `
          (`self.Teleport` (`local.Load`))))
      (else
        (set `local.Load` (`|GetArrayItem` (`/Game/Game/MainGame/SugorokuSystem/Props/Tiles/Tile/BP_TileBase.BeforeTile` (`self.NowTile`))))
        (`/Engine/EditorBlueprintResources/StandardMacros.DecrementInt` (`self.MoveNum`)
          (:`  `
            (`self.Teleport` (`local.Load`))))))
    (if (<= (`self.MoveNum`) 0)
      (if (not (`KismetArrayLibrary.Array_IsEmpty` (`self.Destinations`)))
        (set `self.MoveNum` _movenum)
        (set `local.Load` _load)
        (`KismetArrayLibrary.Array_Remove` (`self.Destinations`))
        (`/Engine/EditorBlueprintResources/StandardMacros.DecrementInt` (`self.MoveNum`)
          (:`  `
            (`self.Teleport` (`local.Load`))
            (return true)))
        (else
          (return true)))
      (else
        (return false)))))

(fn `UserConstructionScript`)