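; Map camera actor for the sugoroku (board game) system that can be panned across the map.
; Four functions (UP, Dawn, Left, Rigft) offset the actor along world X or Y by Speed per call, without sweep or delta-time scaling.
; The event graph and construction script are empty, so the Blueprint handles no input itself and moves only when these functions are called.
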(fn `Dawn`
  (`self.K2_SetActorLocation` (- (`self.K2_GetActorLocation`) (`KismetMathLibrary.MakeVector` (`self.Speed`)))))

(fn `Left`
  (`self.K2_SetActorLocation` (- (`self.K2_GetActorLocation`) (`KismetMathLibrary.MakeVector` 0.0 (`self.Speed`)))))

(fn `Rigft`
  (`self.K2_SetActorLocation` (+ (`self.K2_GetActorLocation`) (`KismetMathLibrary.MakeVector` 0.0 (`self.Speed`)))))

(fn `UP`
  (`self.K2_SetActorLocation` (+ (`self.K2_GetActorLocation`) (`KismetMathLibrary.MakeVector` (`self.Speed`)))))

(fn `UserConstructionScript`)