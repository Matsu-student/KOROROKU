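; Start tile for the sugoroku board game, where pieces are placed at game start.
; SetPieceStartTile registers the given pieces, makes itself their current and next tile, sets their height from box extent, then calls the parent's SetPieceLocation.
; Overlaps keep the piece list and count updated, repositioning pieces when one leaves.
; Entering pieces and BP_TileSercher actors are told this is their current tile.
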(event `self.ReceiveActorBeginOverlap`
  (params (OtherActor :type "Actor Object Reference"))
  (bind _asbp_piece_base (cast `/Game/Game/MainGame/SugorokuSystem/Props/Pieces/BP_PieceBase` OtherActor)
    (:`then`
      (if (not (`KismetArrayLibrary.Array_Contains` (`self.Actors`) _asbp_piece_base))
        (message `/Game/Game/MainGame/SugorokuSystem/Props/Pieces/BI_Piece.SetNowTile` _asbp_piece_base self)
        (`/Engine/EditorBlueprintResources/StandardMacros.IncrementInt` (`self.OnPiece`)
          (:`  `
            (`KismetArrayLibrary.Array_Add` (`self.Actors`) _asbp_piece_base)))))
    (:`CastFailed`
      (bind _asbp_tile_sercher (cast `/Game/Game/MainGame/SugorokuSystem/Props/TileSercher/BP_TileSercher` OtherActor))
      (`/Game/Game/MainGame/SugorokuSystem/Props/TileSercher/BP_TileSercher.SetNowTile` _asbp_tile_sercher self))))

(event `self.ReceiveActorEndOverlap`
  (params (OtherActor :type "Actor Object Reference"))
  (bind _asbp_piece_base (cast `/Game/Game/MainGame/SugorokuSystem/Props/Pieces/BP_PieceBase` OtherActor))
  (if (`KismetArrayLibrary.Array_Contains` (`self.Actors`) _asbp_piece_base)
    (`KismetArrayLibrary.Array_Remove` (`self.Actors`) (`KismetArrayLibrary.Array_Find` (`self.Actors`) _asbp_piece_base))
    (`/Engine/EditorBlueprintResources/StandardMacros.DecrementInt` (`self.OnPiece`)
      (:`  `
        (`self.SetPieceLocation`)))))

(fn `SetPieceLocation`
  (`parent.SetPieceLocation`))

(fn `SetPieceStartTile`
  (params (Pieces :type "Array of /Game/Game/MainGame/SugorokuSystem/Props/Pieces/BP_PieceBase Object Reference"))
  (set `self.Actors` Pieces)
  (for _array_element Pieces
    (set `/Game/Game/MainGame/SugorokuSystem/Props/Pieces/BP_PieceBase.NextTile` self _array_element)
    (set `/Game/Game/MainGame/SugorokuSystem/Props/Pieces/BP_PieceBase.NowTile` self _array_element)
    (bind (_returnvalue_x _returnvalue_y) (`KismetMathLibrary.BreakVector` (`self.K2_GetActorLocation` _array_element)))
    (bind (_returnvalue_x_2 _returnvalue_y_2 _returnvalue_z) (`KismetMathLibrary.BreakVector` (`BoxComponent.GetScaledBoxExtent` (`/Game/Game/MainGame/SugorokuSystem/Props/Pieces/BP_PieceBase.Box` _array_element))))
    (`self.K2_SetActorLocation` _array_element (`KismetMathLibrary.MakeVector` _returnvalue_x _returnvalue_y _returnvalue_z) false false))
  (set `self.OnPiece` (`KismetArrayLibrary.Array_Length` (`self.Actors`)))
  (`self.SetPieceLocation`))

(fn `UserConstructionScript`
  (`parent.UserConstructionScript`))