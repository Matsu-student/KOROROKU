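; BP_TileBase is the base board tile for the Sugoroku system, tracking and arranging the pieces standing on it.
; Overlap events update the piece count and actor list, and send the tile to each arriving actor via SetNowTileMessage.
; SetPieceLocation centres a lone piece or spreads up to four by fixed XY offsets, keeping their Z.
; On arrival, it runs before the new actor joins the list.
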(event `self.ReceiveActorBeginOverlap`
  (params (OtherActor :type "Actor Object Reference"))
  (message `/Game/Game/MainGame/SugorokuSystem/Props/Pieces/BI_Piece.SetNowTile` OtherActor self)
  (`/Engine/EditorBlueprintResources/StandardMacros.IncrementInt` (`self.OnPiece`)
    (:`  `
      (`self.SetPieceLocation`)
      (`KismetArrayLibrary.Array_Add` (`self.Actors`) OtherActor))))

(event `self.ReceiveActorEndOverlap`
  (params (OtherActor :type "Actor Object Reference"))
  (if (> (`self.OnPiece`) 0)
    (`/Engine/EditorBlueprintResources/StandardMacros.DecrementInt` (`self.OnPiece`)
      (:`  `
        (`KismetArrayLibrary.Array_Remove` (`self.Actors`) (`KismetArrayLibrary.Array_Find` (`self.Actors`) OtherActor))
        (`self.SetPieceLocation`)))))

(fn `SetPieceLocation`
  (locals (AddLocation :type "Vector Structure"))
  (bind (_returnvalue_x _returnvalue_y) (`KismetMathLibrary.BreakVector` (`self.K2_GetActorLocation`)))
  (bind (_returnvalue_x_2 _returnvalue_y_2) (`KismetMathLibrary.BreakVector` (+ (`self.K2_GetActorLocation`) (`local.AddLocation`))))
  (if (> (`self.OnPiece`) 0)
    (if (== (`self.OnPiece`) 1)
      (for _array_element (`self.Actors`)
        (bind (_returnvalue_x_3 _returnvalue_y_3 _returnvalue_z) (`KismetMathLibrary.BreakVector` (`self.K2_GetActorLocation` _array_element)))
        (`self.K2_SetActorLocation` _array_element (`KismetMathLibrary.MakeVector` _returnvalue_x _returnvalue_y _returnvalue_z) false false))
      (return)
      (else
        (for (_array_element_2 _array_index) (`self.Actors`)
          (switch `int` _array_index
            (:`0`
              (set `local.AddLocation` (20.0 -40.0 0.0)))
            (:`1`
              (set `local.AddLocation` (30.0 -20.0 0.0)))
            (:`2`
              (set `local.AddLocation` (40.0 20.0 0.0)))
            (:`3`
              (set `local.AddLocation` (50.0 40.0 0.0))))
          (bind (_returnvalue_x_4 _returnvalue_y_4 _returnvalue_z_2) (`KismetMathLibrary.BreakVector` (`self.K2_GetActorLocation` _array_element_2)))
          (`self.K2_SetActorLocation` _array_element_2 (`KismetMathLibrary.MakeVector` _returnvalue_x_2 _returnvalue_y_2 _returnvalue_z_2) false false))
        (return)))
    (else
      (return))))

(fn `UserConstructionScript`)