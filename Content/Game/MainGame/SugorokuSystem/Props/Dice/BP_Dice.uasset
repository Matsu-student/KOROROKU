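; BP_Dice is a dice prop for the Sugoroku board game system that spins and shows random numbers on four widgets.
; BeginPlay caches the four WBP_Dice widgets in an array.
; Each StartRoll call increases spin speed up to a maximum, yaws the cube and pushes a random number within the min/max range to every widget.
; StopRoll displays and returns a fresh random result, then resets the cube's rotation and speed.
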(event `self.ReceiveBeginPlay`
  (bind _aswbp_dice (cast `/Game/Game/MainGame/SugorokuSystem/Props/Dice/WBP_Dice` (`WidgetComponent.GetUserWidgetObject` (`self.Widget0`))))
  (`KismetArrayLibrary.Array_Add` (`self.WBPDice`) _aswbp_dice)
  (bind _aswbp_dice_2 (cast `/Game/Game/MainGame/SugorokuSystem/Props/Dice/WBP_Dice` (`WidgetComponent.GetUserWidgetObject` (`self.Widget1`))))
  (`KismetArrayLibrary.Array_Add` (`self.WBPDice`) _aswbp_dice_2)
  (bind _aswbp_dice_3 (cast `/Game/Game/MainGame/SugorokuSystem/Props/Dice/WBP_Dice` (`WidgetComponent.GetUserWidgetObject` (`self.Widget2`))))
  (`KismetArrayLibrary.Array_Add` (`self.WBPDice`) _aswbp_dice_3)
  (bind _aswbp_dice_4 (cast `/Game/Game/MainGame/SugorokuSystem/Props/Dice/WBP_Dice` (`WidgetComponent.GetUserWidgetObject` (`self.Widget3`))))
  (`KismetArrayLibrary.Array_Add` (`self.WBPDice`) _aswbp_dice_4)
  (for _ (`self.WBPDice`)
    _))

(fn `Result`
  (returns (Number :type Integer))
  (return (`KismetMathLibrary.RandomIntegerInRange` (`self.MinResult`) (`self.MaxResult`))))

(fn `Start Roll`
  (if (< (`self.Rollspeed`) (`self.MaxRollspeed`))
    (bind _output_get (set `self.Rollspeed` (+ (`self.Rollspeed`) 1.0))))
  (`SceneComponent.K2_AddRelativeRotation` (`self.Cube`) (`KismetMathLibrary.MakeRotator` 0.0 0.0 _output_get) false false)
  (bind _number (`self.Result`))
  (for _array_element (`self.WBPDice`)
    (`/Game/Game/MainGame/SugorokuSystem/Props/Dice/WBP_Dice.SetNum` _array_element _number)))

(fn `StopRoll`
  (returns (Number :type Integer))
  (bind _number (`self.Result`))
  (for _array_element (`self.WBPDice`)
    (`/Game/Game/MainGame/SugorokuSystem/Props/Dice/WBP_Dice.SetNum` _array_element _number))
  (`SceneComponent.K2_SetRelativeRotation` :`self` (`self.Cube`))
  (set `self.Rollspeed` 0.0)
  (return _number))

(fn `UserConstructionScript`)