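; Base card deck for the sugoroku card game, supplying random cards as WBP_DebugCard widgets.
; On BeginPlay it copies every DTCardDeck row into CardDeck and sets CanUse once 30 cards are loaded.
; DrawCard re-rolls random indices until a slot has IsUse set, then passes its type and matching effect to the widget.
; IsUse is cleared only on the CardDeckSlot copy, never written back to the array.
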(event `self.ReceiveBeginPlay`
  (`self.CreateCardDeck`))

(fn `CreateCardDeck`
  (if (!= (`self.DT_CardDeck`) null)
    (bind _outrownames (`DataTableFunctionLibrary.GetDataTableRowNames` (`self.DT_CardDeck`)))
    (for _array_element _outrownames
      (bind _returnvalue (`|GetDataTableRow` (`self.DT_CardDeck`) _array_element)
        (:`then`
          (bind _returnvalue_2 (`KismetArrayLibrary.Array_Add` (`self.CardDeck`) _returnvalue))
          (set `self.CanUse` (>= _returnvalue_2 29)) ; 使えるようになった
        )))))

(fn `DrawCard`
  (returns (ReturnValue :type "/Game/Game/MainGame/SugorokuSystem/CardGameSystem/Card/Cards/WBP_DebugCard Object Reference"))
  (locals (Rand :type Integer) (IsDrawCrad :type Boolean) (CardDeckSlot :type "/Game/Game/MainGame/SugorokuSystem/CardGameSystem/Card/CardDeck/F_CardDeckSlot Structure"))
  (set `local.Rand` (`KismetMathLibrary.RandomIntegerInRange` 0 (`self.CardMax`)) :!label _label)
  (for (_array_element _array_index) (`self.CardDeck`)
    (if (== _array_index (`local.Rand`))
      (bind _output_get (set `local.CardDeckSlot` _array_element))
      (bind (_isuse _type _effect0 _effect1 _effect2 _effect3) (break `/Game/Game/MainGame/SugorokuSystem/CardGameSystem/Card/CardDeck/F_CardDeckSlot` _output_get))
      (if _isuse
        (set `local.CardDeckSlot` (make `/Game/Game/MainGame/SugorokuSystem/CardGameSystem/Card/CardDeck/F_CardDeckSlot` false _type _effect0 _effect1 _effect2 _effect3))
        (bind _returnvalue (`|CreateWidget` "/Game/Game/MainGame/SugorokuSystem/CardGameSystem/Card/Cards/WBP_DebugCard.WBP_DebugCard_C"))
        (set `/Game/Game/MainGame/SugorokuSystem/CardGameSystem/Card/Cards/CardBase/WBP_CardBase.CardType` _type _returnvalue)
        (switch `/Game/Game/MainGame/SugorokuSystem/CardGameSystem/Card/Cards/CardBase/Data/E_CardType` _type
          (:`NewEnumerator0`
            (if (!= _effect0 0)
              (set `/Game/Game/MainGame/SugorokuSystem/CardGameSystem/Card/Cards/CardBase/WBP_CardBase.CardEffect` (`KismetMathLibrary.Conv_ByteToInt` _effect0) _returnvalue)
              (return _returnvalue)
              (else
                _)))
          (:`NewEnumerator1`
            (if (!= _effect1 0)
              (set `/Game/Game/MainGame/SugorokuSystem/CardGameSystem/Card/Cards/CardBase/WBP_CardBase.CardEffect` (`KismetMathLibrary.Conv_ByteToInt` _effect1) _returnvalue)
              (return _returnvalue)
              (else
                _)))
          (:`NewEnumerator2`
            (if (!= _effect2 0)
              (set `/Game/Game/MainGame/SugorokuSystem/CardGameSystem/Card/Cards/CardBase/WBP_CardBase.CardEffect` (`KismetMathLibrary.Conv_ByteToInt` _effect2) _returnvalue)
              (return _returnvalue)
              (else
                _)))
          (:`NewEnumerator3`
            (if (!= _effect3 0)
              (set `/Game/Game/MainGame/SugorokuSystem/CardGameSystem/Card/Cards/CardBase/WBP_CardBase.CardEffect` (`KismetMathLibrary.Conv_ByteToInt` _effect3) _returnvalue)
              (return _returnvalue)
              (else
                _))))
        (set `local.IsDrawCrad` true)
        (`KismetSystemLibrary.PrintString` "CradDrawErrer")
        (else
          (goto _label)))))
  (if (`local.IsDrawCrad`)
    (return null)
    (else
      (goto _label))))

(fn `UserConstructionScript`)