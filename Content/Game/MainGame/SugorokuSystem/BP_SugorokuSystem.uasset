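; BP_SugorokuSystem runs the main loop of a sugoroku board game.
; BeginPlay spawns a piece per player, places them on the start tile and creates a TileEffectPlayer.
; Each tick runs the data-table-driven task queue, which is shared with the card game component.
; When tasks finish, it switches player, requeues tasks, moves the camera to that player's piece and advances the turn counter on a hardcoded four-player threshold.
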(event `self.ReceiveBeginPlay`
  ;[1 1 1] Player分のコマを作成する
  (for (_array_element _array_index) (`GameStateBase.PlayerArray` (`GameplayStatics.GetGameState`))
    (message `/Game/Game/MainGame/SugorokuSystem/PlayerState/BI_SugorokuPS.Set PlayerNumber` _array_element _array_index)
    (bind _returnvalue (`|SpawnActorFromClass` "/Game/Game/MainGame/SugorokuSystem/Props/Pieces/BP_PieceBase.BP_PieceBase_C" (`KismetMathLibrary.MakeTransform` (0.0 0.0 0.0)) "Undefined" "MultiplyWithRoot" null null))
    (set `/Game/Game/MainGame/SugorokuSystem/Props/Pieces/BP_PieceBase.PlayerID` _array_index _returnvalue) ; コマにplayerのＩＤを登録
  )
  ;;[1 1 1] スゴロクシステムがコマを保管
  (bind _outactors (`GameplayStatics.GetAllActorsOfClass` "/Game/Game/MainGame/SugorokuSystem/Props/Pieces/BP_PieceBase.BP_PieceBase_C"))
  (set `self.Pieces` _outactors)
  ;[1 1 1] カメラ切り替え
  ;;[1 1 1] 現在のプレイヤーを取得
  (bind _nowplayernumber (message `/Game/Game/MainGame/SugorokuSystem/GameLoop/PlayerSwitcher/BI_PlayerSwitcher.GetNowPlayerNumber` (`self.AC_PlayerSwitcher`)))
  (set `self.NowPlayerNumber` _nowplayernumber)
  ;;[1 1 1] カメラを現在のプレイヤーのコマに切り替える
  (`self.SwitchNowPlayerPieceCamera`)
  ;[1 1 1] スタートマスにコマを設置
  (bind _returnvalue_2 (`GameplayStatics.GetActorOfClass` "/Game/Game/MainGame/SugorokuSystem/Props/Tiles/BP_StartTile.BP_StartTile_C"))
  (`/Game/Game/MainGame/SugorokuSystem/Props/Tiles/BP_StartTile.SetPieceStartTile` _returnvalue_2 (`self.Pieces`))
  ;[1 1 1] TileEffectPlayerを作成してスゴロクシステムで保管
  (bind _returnvalue_3 (`|SpawnActorFromClass` "/Game/Game/MainGame/SugorokuSystem/GameLoop/TileEffectPlayer/BP_TileEffectPlayer.BP_TileEffectPlayer_C" (`self.GetTransform` self) "Undefined" "MultiplyWithRoot" null null))
  (set `self.TileEffectPlayer` _returnvalue_3)
  ;[1 1 1] 初回タスクを予約
  (`self.AddMainLoopTask`)
  ;[1 1 1] CardGameSystemでもTaskの予約を許可
  (set `/Game/Game/MainGame/SugorokuSystem/CardGameSystem/AC_CardGameSystem.TaskPlayer` (`self.AC_TaskPlayer`) (`self.AC_CardGameSystem`)))

(event `self.ReceiveTick`
  (params (DeltaSeconds :type "Float (single-precision)"))
  ;[1 1 1] Taskを実行
  (bind _isendplay (`/Game/Game/MainGame/SugorokuSystem/GameLoop/Task/TaskPlayer/AC_TaskPlayer.Process` (`self.AC_TaskPlayer`) (`self.NowPlayerNumber`)))
  ;[1 1 1] CardGameSystemの処理
  (`/Game/Game/MainGame/SugorokuSystem/CardGameSystem/AC_CardGameSystem.Process` (`self.AC_CardGameSystem`) (`self.NowPlayerNumber`))
  ;[1 1 1] プレイヤーを切り替える
  (if _isendplay
    (bind (_nowplayerid _playernum) (`/Game/Game/MainGame/SugorokuSystem/GameLoop/PlayerSwitcher/AC_PlayerSwitcher.SwitchPlayer` (`self.AC_PlayerSwitcher`)))
    (set `self.NowPlayerNumber` _nowplayerid)
    ;[1 1 1] 次のプレイヤーの準備
    (`self.AddMainLoopTask`)
    ;[1 1 1] カメラを現在のプレイヤーのコマに切り替える
    (`self.SwitchNowPlayerPieceCamera`)
    ;[1 1 1] ターンを進める
    (if (>= _playernum 3)
      (`/Game/Game/MainGame/SugorokuSystem/GameLoop/TurnCounter/AC_TurnUPCounter.Play` (`self.AC_TurnUPCounter`)))))

(fn `AddMainLoopTask`
  ;[1 1 1] データテーブルに登録されたタスクを予約する
  (if (!= (`self.MainLoopTask`) null)
    ;;[1 1 1] データテーブルを読み出す
    (bind _outrownames (`DataTableFunctionLibrary.GetDataTableRowNames` (`self.MainLoopTask`)))
    (for _array_element _outrownames
      (bind _returnvalue (`|GetDataTableRow` (`self.MainLoopTask`) _array_element)
        (:`then`
          (`/Game/Game/MainGame/SugorokuSystem/GameLoop/Task/TaskPlayer/AC_TaskPlayer.Add` (`self.AC_TaskPlayer`) (`.Task_2_3FFA80024F41657DB96CBBB8DF64A3C0` (break `/Game/Game/MainGame/SugorokuSystem/GameLoop/Task/MainTaskLoop/F_TaskName` _returnvalue))))))
    (return)
    (else
      (`KismetSystemLibrary.PrintString` "Error/データテーブルが選択されていませんでした"))))

(fn `GetNowPlayerPiece`
  (returns (Piece :type "/Game/Game/MainGame/SugorokuSystem/Props/Pieces/BP_PieceBase Object Reference"))
  (for _array_element (`self.Pieces`)
    (if (== (`/Game/Game/MainGame/SugorokuSystem/Props/Pieces/BP_PieceBase.PlayerID` _array_element) (`self.NowPlayerNumber`))
      (break)))
  (return _array_element))

(fn `Init`)

(fn `SwitchNowPlayerPieceCamera`
  (bind _piece (`self.GetNowPlayerPiece`))
  (`/Game/Game/MainGame/SugorokuSystem/GameLoop/CameraSwitcher/AC_CameraSwitcher.SwitchCamera` (`self.AC_CameraSwitcher`) _piece)
  (return))

(fn `UserConstructionScript`)