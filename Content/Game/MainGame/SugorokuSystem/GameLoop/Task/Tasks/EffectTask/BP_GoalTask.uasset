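; BP_GoalTask is a sugoroku game-loop effect task that handles the current player's piece on a goal tile.
; On init it finds the piece matching the current player number and caches its tile.
; TaskPlay calls AddGItemMessage on the player state's ItemTeller, then checks a 60-frame wait.
; Once the wait completes it destroys the goal object, clears the tile's effect and stop flag, and queues SetGoal and Move tasks.
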(event `/Game/Game/MainGame/SugorokuSystem/GameLoop/Task/Tasks/TaskBase/BI_Task.TaskInit`
  (bind _outactors (`GameplayStatics.GetAllActorsOfClass` "/Game/Game/MainGame/SugorokuSystem/Props/Pieces/BP_PieceBase.BP_PieceBase_C"))
  (for _array_element _outactors
    (bind _playernumber (message `/Game/Game/MainGame/SugorokuSystem/Props/Pieces/BI_Piece.GetPlayerNumber` _array_element))
    (if (== _playernumber (`self.NowPlayerNumber`))
      (set `self.Now Tile` (`/Game/Game/MainGame/SugorokuSystem/Props/Pieces/BP_PieceBase.NowTile` _array_element)))))

(fn `Insert Task`
  (params (TaskName :type Name) (Index :type Integer) (Number :type Integer))
  (`parent.Insert Task` TaskName Index Number))

(fn `TaskPlay`
  (returns (isTaskEnd :type Boolean))
  (bind _now_tile (`self.Now Tile`))
  (bind _asbp_sugoroku_ps (cast `/Game/Game/MainGame/SugorokuSystem/PlayerState/BP_SugorokuPS` (`self.PlayerState`)))
  (message `/Game/Game/MainGame/SugorokuSystem/ItemStrage/BI_ItemIO.AddGItem` (`/Game/Game/MainGame/SugorokuSystem/PlayerState/BP_SugorokuPS.ItemTeller` _asbp_sugoroku_ps) 1)
  (bind _end (`self.Wait` 60))
  (if _end
    (`self.K2_DestroyActor` (`/Game/Game/MainGame/SugorokuSystem/Props/Tiles/Tile/BP_TileBase.GoalObj` _now_tile))
    (set `/Game/Game/MainGame/SugorokuSystem/Props/Tiles/Tile/BP_TileBase.AddEffect` "None" _now_tile)
    (set `/Game/Game/MainGame/SugorokuSystem/Props/Tiles/Tile/BP_TileBase.IsStop` false _now_tile)
    (`self.Insert Task` "SetGoal" 0 1)
    (`self.Insert Task` "Move" 1 1))
  (return _end))

(fn `UserConstructionScript`
  (`parent.UserConstructionScript`))

(fn `Wait`
  (params (Frame :type Integer))
  (returns (End :type Boolean))
  (bind _end (`parent.Wait` Frame))
  (return _end))