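; Effect task in the sugoroku game loop that handles the combo attack manager's cleanup.
; TaskInit finds and caches the BP_ComboAttackManeger actor already in the level, and TaskFina destroys it after a reference check.
; TaskPlay does no work and immediately returns true, so the task itself runs no attack logic.
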(event `/Game/Game/MainGame/SugorokuSystem/GameLoop/Task/Tasks/TaskBase/BI_Task.TaskInit`
  (bind _returnvalue (`GameplayStatics.GetActorOfClass` "/Game/Game/MainGame/SugorokuSystem/Props/ComboAttackManeger/BP_ComboAttackManeger.BP_ComboAttackManeger_C"))
  (set `self.ComboAttackManeger` _returnvalue))

(event `/Game/Game/MainGame/SugorokuSystem/GameLoop/Task/Tasks/TaskBase/BI_Task.TaskFina`
  (if (!= (`self.ComboAttackManeger`) null)
    (`self.K2_DestroyActor` (`self.ComboAttackManeger`))))

(fn `TaskPlay`
  (returns (isTaskEnd :type Boolean))
  (return true))

(fn `UserConstructionScript`
  (`parent.UserConstructionScript`))