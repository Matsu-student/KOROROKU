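; BP_DebugRangeTask is a debug effect task in the sugoroku board game loop that picks target tiles around the current player's piece.
; On init it spawns a BP_TileSercher with a move count of three, seeded at the tile of the piece matching the current player number.
; Each play polls the searcher's TeleportNextTile; on success it hands the searched tiles to the combo attack manager and completes.
; The searcher is destroyed when the task finishes.
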(event `self.TaskInit`
  (bind _returnvalue (`GameplayStatics.GetActorOfClass` "/Game/Game/MainGame/SugorokuSystem/Props/ComboAttackManeger/BP_ComboAttackManeger.BP_ComboAttackManeger_C"))
  (set `self.ComboAttackManeger` _returnvalue)
  (bind _returnvalue_2 (`|SpawnActorFromClass` "/Game/Game/MainGame/SugorokuSystem/Props/TileSercher/BP_TileSercher.BP_TileSercher_C" (`KismetMathLibrary.MakeTransform` (0.0 0.0 -1000.0)) "Undefined" "MultiplyWithRoot" null null))
  (bind _output_get (set `self.TileSercher` _returnvalue_2))
  (set `/Game/Game/MainGame/SugorokuSystem/Props/TileSercher/BP_TileSercher.MoveNum` 3 _output_get)
  (bind _outactors (`GameplayStatics.GetAllActorsOfClass` "/Game/Game/MainGame/SugorokuSystem/Props/Pieces/BP_PieceBase.BP_PieceBase_C"))
  (for _array_element _outactors
    (if (== (`/Game/Game/MainGame/SugorokuSystem/Props/Pieces/BP_PieceBase.PlayerNumber` _array_element) (`self.NowPlayerNumber`))
      (set `self.Piece` _array_element)
      (break)))
  (`/Game/Game/MainGame/SugorokuSystem/Props/TileSercher/BP_TileSercher.SetNowTile` (`self.TileSercher`) (`/Game/Game/MainGame/SugorokuSystem/Props/Pieces/BP_PieceBase.NowTile` (`self.Piece`))))

(event `/Game/Game/MainGame/SugorokuSystem/GameLoop/Task/Tasks/TaskBase/BI_Task.TaskFina`
  (`self.K2_DestroyActor` (`self.TileSercher`)))

(fn `TaskPlay`
  (returns (isTaskEnd :type Boolean))
  (bind _serchend (`/Game/Game/MainGame/SugorokuSystem/Props/TileSercher/BP_TileSercher.TeleportNextTile` (`self.TileSercher`)))
  (if _serchend
    (set `/Game/Game/MainGame/SugorokuSystem/Props/ComboAttackManeger/BP_ComboAttackManeger.TargetTiles` (`/Game/Game/MainGame/SugorokuSystem/Props/TileSercher/BP_TileSercher.SerchTiles` (`self.TileSercher`)) (`self.ComboAttackManeger`))
    (return true)
    (else
      (return false))))

(fn `UserConstructionScript`
  (`parent.UserConstructionScript`))