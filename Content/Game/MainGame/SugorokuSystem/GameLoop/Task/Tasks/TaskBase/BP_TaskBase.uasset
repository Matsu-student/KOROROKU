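; BP_TaskBase is the base Blueprint for tasks in the Sugoroku game loop, with empty init and finish events and a placeholder TaskPlay returning true.
; Setters inject player state, controller, player number and card game system, while input events forward to the PlayerState's UI messages.
; Helpers provide frame-count waits, a repeat-call check, scene ID access, and queued task insertion requests exposed through GetInsertTask.
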(event `/Game/Game/MainGame/SugorokuSystem/PlayerController/BI_SugorokuPC.Decide`
  (params (Input :type Boolean))
  (message `/Game/Game/MainGame/SugorokuSystem/PlayerState/BI_SugorokuPS.UIDecide` (`self.PlayerState`)))

(event `/Game/Game/MainGame/SugorokuSystem/GameLoop/Task/Tasks/TaskBase/BI_Task.SetNowPlayerNumber`
  (params (PlayerNumber :type Integer))
  (set `self.NowPlayerNumber` PlayerNumber))

(event `/Game/Game/MainGame/SugorokuSystem/GameLoop/Task/Tasks/TaskBase/BI_Task.TaskInit`)

(event `/Game/Game/MainGame/SugorokuSystem/PlayerController/BI_SugorokuPC.Cancel`
  (params (Input :type Boolean))
  (message `/Game/Game/MainGame/SugorokuSystem/PlayerState/BI_SugorokuPS.UICancel` (`self.PlayerState`)))

(event `/Game/Game/MainGame/SugorokuSystem/PlayerController/BI_SugorokuPC.SetPlayerContller`
  (params (PlayerContller :type "PlayerController Object Reference"))
  (set `self.Player Contller` PlayerContller))

(event `/Game/Game/MainGame/SugorokuSystem/GameLoop/Task/Tasks/TaskBase/BI_Task.TaskFina`)

(event `/Game/Game/MainGame/SugorokuSystem/PlayerController/BI_SugorokuPC.UP`
  (params (Input :type Boolean))
  (message `/Game/Game/MainGame/SugorokuSystem/PlayerState/BI_SugorokuPS.UIUP` (`self.PlayerState`)))

(event `/Game/Game/MainGame/SugorokuSystem/GameLoop/Task/Tasks/TaskBase/BI_Task.SetCardGameSytem`
  (params (CardGameSystem :type "ActorComponent Object Reference"))
  (set `self.Card Game System` CardGameSystem))

(event `/Game/Game/MainGame/SugorokuSystem/PlayerController/BI_SugorokuPC.Dawn`
  (params (Input :type Boolean))
  (message `/Game/Game/MainGame/SugorokuSystem/PlayerState/BI_SugorokuPS.UIDawn` (`self.PlayerState`)))

(event `/Game/Game/MainGame/SugorokuSystem/GameLoop/Task/Tasks/TaskBase/BI_Task.GetOutputDataNum`
  (params (DataNum :type Integer))
  (set `self.OutputDataNum` DataNum))

(event `/Game/Game/MainGame/SugorokuSystem/PlayerController/BI_SugorokuPC.left`
  (params (Input :type Boolean))
  (message `/Game/Game/MainGame/SugorokuSystem/PlayerState/BI_SugorokuPS.UILeft` (`self.PlayerState`)))

(event `/Game/Game/MainGame/SugorokuSystem/GameLoop/Task/Tasks/TaskBase/BI_Task.SetPlayerState`
  (params (PlayerState :type "PlayerState Object Reference"))
  (set `self.PlayerState` PlayerState))

(event `/Game/Game/MainGame/SugorokuSystem/PlayerController/BI_SugorokuPC.Right`
  (params (Input :type Boolean))
  (message `/Game/Game/MainGame/SugorokuSystem/PlayerState/BI_SugorokuPS.UIRight` (`self.PlayerState`)))

(fn `GetInsertTask`
  (returns (TaskName :type "Array of Name") (Index :type "Array of Integer") (Number :type "Array of Integer") (IsInsertTask :type Boolean))
  (return (`self.InsertTaskName`) (`self.InsertIndex`) (`self.Number`) (`self.IsInsertTask`)))

(fn `GetSceneID`
  (returns (SceneID :type Integer))
  (return (`self.ViewSceneID`)))

(fn `Insert Task`
  (params (TaskName :type Name) (Index :type Integer) (Number :type Integer))
  (`KismetArrayLibrary.Array_Add` (`self.InsertTaskName`) TaskName)
  (`KismetArrayLibrary.Array_Add` (`self.InsertIndex`) Index)
  (`KismetArrayLibrary.Array_Add` (`self.Number`) Number)
  (if (not (`self.IsInsertTask`))
    (set `self.IsInsertTask` true))
  (return))

(fn `Once`
  (returns (IsUse :type Boolean))
  (locals (over :type Boolean :default false))
  (set `local.over` (> (`self.countUse`) 0))
  (`/Engine/EditorBlueprintResources/StandardMacros.IncrementInt` (`self.countUse`)
    (:`  `
      (return (`local.over`)))))

(fn `TaskPlay`
  (returns (isTaskEnd :type Boolean))
  (`KismetSystemLibrary.PrintString` (`KismetStringLibrary.Concat_StrStr` (`KismetStringLibrary.Conv_NameToString` (`self.Key`)) "/" "Play") true true (struct :`G` 0.66 :`B` 1.0 :`A` 1.0) 10.0 (`self.Key`))
  (return true))

(fn `UserConstructionScript`)

(fn `Wait`
  (params (Frame :type Integer))
  (returns (End :type Boolean))
  (bind _result (`/Engine/EditorBlueprintResources/StandardMacros.IncrementInt` (`self.CountFrame`))
    (:`  `
      (`KismetSystemLibrary.PrintString` (`KismetStringLibrary.Conv_IntToString` _result) true true (struct :`R` 1.0 :`B` 0.419177 :`A` 1.0) 2.0 "WaitTimer")
      (if (>= (`self.CountFrame`) Frame)
        (set `self.CountFrame` 0)
        (return true)
        (else
          (return false))))))