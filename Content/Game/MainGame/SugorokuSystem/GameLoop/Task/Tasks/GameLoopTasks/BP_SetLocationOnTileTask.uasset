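; Game loop task for the sugoroku board game that places the current player's piece on its tile.
; It caches every BP_PieceBase actor at BeginPlay.
; TaskPlay finds the piece matching NowPlayerNumber, calls InitMove on it, has its current tile set piece locations, then sets the piece's location on that tile.
; The task always returns true immediately.
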(event `self.ReceiveBeginPlay`
  (`parent.ReceiveBeginPlay`)
  (bind _outactors (`GameplayStatics.GetAllActorsOfClass` "/Game/Game/MainGame/SugorokuSystem/Props/Pieces/BP_PieceBase.BP_PieceBase_C"))
  (set `self.Pieces` _outactors))

(fn `TaskPlay`
  (returns (isTaskEnd :type Boolean))
  (for _array_element (`self.Pieces`)
    (if (== (`/Game/Game/MainGame/SugorokuSystem/Props/Pieces/BP_PieceBase.PlayerNumber` _array_element) (`self.NowPlayerNumber`))
      (`/Game/Game/MainGame/SugorokuSystem/Props/Pieces/BP_PieceBase.InitMove` _array_element)
      (`/Game/Game/MainGame/SugorokuSystem/Props/Tiles/Tile/BP_TileBase.SetPieceLocation` (`/Game/Game/MainGame/SugorokuSystem/Props/Pieces/BP_PieceBase.NowTile` _array_element))
      (`/Game/Game/MainGame/SugorokuSystem/Props/Pieces/BP_PieceBase.SetLoacationOnTile` _array_element)
      (break)))
  (return true))

(fn `UserConstructionScript`
  (`parent.UserConstructionScript`))