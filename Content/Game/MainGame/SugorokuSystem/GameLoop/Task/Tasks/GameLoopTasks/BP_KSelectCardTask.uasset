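; Game loop task for the sugoroku board game in which the player selects a card.
; On init it switches the player to Game and UI input, then tells the card game system to show the cards and start card selection.
; The play step reports completion once the output data number is non-zero, and teardown restores game-only input.
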(event `/Game/Game/MainGame/SugorokuSystem/GameLoop/Task/Tasks/TaskBase/BI_Task.TaskInit`
  (`WidgetBlueprintLibrary.SetInputMode_GameAndUIEx` (`self.Player Contller`) null "DoNotLock" true true)
  (message `/Game/Game/MainGame/SugorokuSystem/CardGameSystem/BI_CardGameSystem.OrderViewCards` (`self.Card Game System`))
  (message `/Game/Game/MainGame/SugorokuSystem/CardGameSystem/BI_CardGameSystem.OrderInitCardSelect` (`self.Card Game System`)))

(event `/Game/Game/MainGame/SugorokuSystem/GameLoop/Task/Tasks/TaskBase/BI_Task.TaskFina`
  (`WidgetBlueprintLibrary.SetInputMode_GameOnly` (`self.Player Contller`)))

(fn `TaskPlay`
  (returns (isTaskEnd :type Boolean))
  (return (!= (`self.OutputDataNum`) 0)))

(fn `UserConstructionScript`
  (`parent.UserConstructionScript`))