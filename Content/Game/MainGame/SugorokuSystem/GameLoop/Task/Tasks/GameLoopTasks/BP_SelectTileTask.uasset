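; Game loop task in a sugoroku board game that lets the current player choose the next tile to move to.
; On init it finds the piece matching the current player number and enables Game and UI input, restoring game-only input on finish.
; TaskPlay does a one-time setup of a scene button per NextTile of the piece's tile.
; Once OutputDataNum is positive, it sets the piece's LoadIndex and completes when SelectMove succeeds.
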(event `self.ReceiveBeginPlay`
  (`parent.ReceiveBeginPlay`))

(event `/Game/Game/MainGame/SugorokuSystem/GameLoop/Task/Tasks/TaskBase/BI_Task.TaskInit`
  (`parent.TaskInit`)
  (bind _outactors (`GameplayStatics.GetAllActorsOfClass` "/Game/Game/MainGame/SugorokuSystem/Props/Pieces/BP_PieceBase.BP_PieceBase_C"))
  (for _array_element _outactors
    (if (== (`/Game/Game/MainGame/SugorokuSystem/Props/Pieces/BP_PieceBase.PlayerID` _array_element) (`self.NowPlayerNumber`))
      (set `self.Piece` _array_element)
      (break)))
  (`WidgetBlueprintLibrary.SetInputMode_GameAndUIEx` (`self.Player Contller`) null "DoNotLock" true true))

(event `/Game/Game/MainGame/SugorokuSystem/GameLoop/Task/Tasks/TaskBase/BI_Task.TaskFina`
  (`parent.TaskFina`)
  (`WidgetBlueprintLibrary.SetInputMode_GameOnly` (`self.Player Contller`) true))

(fn `Once`
  (returns (IsUse :type Boolean))
  (bind _isuse (`parent.Once`))
  (return _isuse))

(fn `TaskPlay`
  (returns (isTaskEnd :type Boolean))
  (bind _outputdatanum (`self.OutputDataNum`))
  (bind _isuse (`self.Once` :!label _label))
  (if _isuse
    (if (> _outputdatanum 0)
      (set `/Game/Game/MainGame/SugorokuSystem/Props/Pieces/BP_PieceBase.LoadIndex` (- _outputdatanum 1) (`self.Piece`))
      (bind _end (`/Game/Game/MainGame/SugorokuSystem/Props/Pieces/BP_PieceBase.SelectMove` (`self.Piece`)))
      (if _end
        (return true)
        (else
          (return false)))
      (else
        (return false)))
    (else
      (`/Game/Game/MainGame/SugorokuSystem/Props/Pieces/BP_PieceBase.InitMove` (`self.Piece`))
      (for (_ _array_index) (`/Game/Game/MainGame/SugorokuSystem/Props/Tiles/Tile/BP_TileBase.NextTile` (`/Game/Game/MainGame/SugorokuSystem/Props/Pieces/BP_PieceBase.NowTile` (`self.Piece`)))
        (bind _returnvalue (`|CreateWidget` "/Game/Game/MainGame/SugorokuSystem/UI/Props/WBP_SugorokuBotton.WBP_SugorokuBotton_C"))
        (set `/Game/Game/MainGame/SugorokuSystem/UI/Props/WBP_SugorokuBotton.InputNumber` _array_index _returnvalue)
        (set `/Game/Game/MainGame/SugorokuSystem/UI/Props/WBP_SugorokuBotton.Task` self _returnvalue)
        (bind _aswbp_select_tile_scene (cast `/Game/Game/MainGame/SugorokuSystem/UI/Scene/SelectTileScene/WBP_SelectTileScene` (`self.Scene Widget`))
          (:`then`
            (`/Game/Game/MainGame/SugorokuSystem/UI/Scene/SelectTileScene/WBP_SelectTileScene.SetSugorokuButton` _aswbp_select_tile_scene _returnvalue))
          (:`CastFailed`
            (`Widget.RemoveFromParent` _returnvalue))))
      (goto _label))))

(fn `UserConstructionScript`
  (`parent.UserConstructionScript`))