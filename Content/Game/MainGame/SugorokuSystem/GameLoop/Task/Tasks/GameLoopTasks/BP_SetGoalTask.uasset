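; BP_SetGoalTask is a sugoroku game-loop task that places a new goal on a random board tile and shows it to the player.
; On init it counts existing goals, and if there are at most four, picks a non-start, non-goal tile, spawns a goal object and camera there, and marks it as a stopping Goal tile.
; After a fixed frame wait, it returns the view to the current player's piece and destroys the goal camera.
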(event `/Game/Game/MainGame/SugorokuSystem/GameLoop/Task/Tasks/TaskBase/BI_Task.TaskInit`
  (bind _goal (`self.Goal`))
  (bind _targettile (`self.TargetTile`))
  (bind _returnvalue (`self.GetTransform` (`self.TargetTile`)))
  (bind _outactors (`GameplayStatics.GetAllActorsOfClass` "/Game/Game/MainGame/SugorokuSystem/Props/Pieces/BP_PieceBase.BP_PieceBase_C"))
  (for _array_element _outactors
    (if (== (`/Game/Game/MainGame/SugorokuSystem/Props/Pieces/BP_PieceBase.PlayerNumber` _array_element) (`self.NowPlayerNumber`))
      (set `self.ViewTaget` _array_element)
      (break)))
  (bind _returnvalue_2 (`GameplayStatics.GetActorOfClass` "/Game/Game/MainGame/SugorokuSystem/BP_SugorokuSystem.BP_SugorokuSystem_C"))
  (set `self.CameraSwitcher` (`self.GetComponentByClass` _returnvalue_2 "/Game/Game/MainGame/SugorokuSystem/GameLoop/CameraSwitcher/AC_CameraSwitcher.AC_CameraSwitcher_C"))
  (bind _outactors_2 (`GameplayStatics.GetAllActorsOfClass` "/Game/Game/MainGame/SugorokuSystem/Props/Tiles/Tile/BP_TileBase.BP_TileBase_C"))
  (for _array_element_2 _outactors_2
    (if (== (`/Game/Game/MainGame/SugorokuSystem/Props/Tiles/Tile/BP_TileBase.AddEffect` _array_element_2) "Goal")
      (`/Engine/EditorBlueprintResources/StandardMacros.IncrementInt` (`self.GoalNum`))
      (elif (!= _array_element_2 "/Game/Game/MainGame/SugorokuSystem/Props/Tiles/BP_StartTile.BP_StartTile")
        (`KismetArrayLibrary.Array_Add` (`self.Goal`) _array_element_2))))
  (if (<= (`self.GoalNum`) 4)
    (set `self.TargetTile` (`|GetArrayItem` _goal (`KismetMathLibrary.RandomInteger` (`KismetArrayLibrary.Array_Length` _goal))))
    (bind _returnvalue_3 (`|SpawnActorFromClass` "/Game/Game/MainGame/SugorokuSystem/Props/GoalCamera/BP_GoalCamera.BP_GoalCamera_C" _returnvalue "Undefined" "MultiplyWithRoot" null null))
    (set `self.GoalCamera` _returnvalue_3)
    (`/Game/Game/MainGame/SugorokuSystem/GameLoop/CameraSwitcher/AC_CameraSwitcher.SwitchCamera` (`self.CameraSwitcher`) (`self.GoalCamera`))
    (bind _returnvalue_4 (`|SpawnActorFromClass` "/Game/Game/MainGame/SugorokuSystem/Props/Goal/BP_GoalObj.BP_GoalObj_C" _returnvalue "Undefined" "MultiplyWithRoot" null null))
    (set `/Game/Game/MainGame/SugorokuSystem/Props/Tiles/Tile/BP_TileBase.GoalObj` _returnvalue_4 _targettile)
    (set `/Game/Game/MainGame/SugorokuSystem/Props/Tiles/Tile/BP_TileBase.AddEffect` "Goal" _targettile)
    (set `/Game/Game/MainGame/SugorokuSystem/Props/Tiles/Tile/BP_TileBase.IsStop` true _targettile)))

(event `/Game/Game/MainGame/SugorokuSystem/GameLoop/Task/Tasks/TaskBase/BI_Task.TaskFina`
  (`/Game/Game/MainGame/SugorokuSystem/GameLoop/CameraSwitcher/AC_CameraSwitcher.SwitchCamera` (`self.CameraSwitcher`) (`self.ViewTaget`))
  (`self.K2_DestroyActor` (`self.GoalCamera`)))

(fn `TaskPlay`
  (returns (isTaskEnd :type Boolean))
  (bind _end (`self.Wait` 100))
  (return _end))

(fn `UserConstructionScript`
  (`parent.UserConstructionScript`))

(fn `Wait`
  (params (Frame :type Integer))
  (returns (End :type Boolean))
  (bind _end (`parent.Wait` Frame))
  (return _end))