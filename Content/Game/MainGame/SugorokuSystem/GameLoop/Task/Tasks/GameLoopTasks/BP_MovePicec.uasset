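; Game loop task that moves the current player's piece in the Sugoroku board game.
; TaskInit searches all BP_PieceBase actors for the one matching NowPlayerNumber, caches it and calls InitMove on it.
; TaskPlay delegates to the piece's Move, inserting a SelectTile task when it reports CanSelect, and returns its End flag as the task result.
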(event `/Game/Game/MainGame/SugorokuSystem/GameLoop/Task/Tasks/TaskBase/BI_Task.TaskInit`
  (bind _outactors (`GameplayStatics.GetAllActorsOfClass` "/Game/Game/MainGame/SugorokuSystem/Props/Pieces/BP_PieceBase.BP_PieceBase_C"))
  (set `self.Pieces` _outactors)
  (for _array_element (`self.Pieces`)
    (if (== (`/Game/Game/MainGame/SugorokuSystem/Props/Pieces/BP_PieceBase.PlayerNumber` _array_element) (`self.NowPlayerNumber`))
      (set `self.Piece` _array_element)
      (`/Game/Game/MainGame/SugorokuSystem/Props/Pieces/BP_PieceBase.InitMove` (`self.Piece`))
      (break))))

(fn `GetInsertTask`
  (returns (TaskName :type "Array of Name") (Index :type "Array of Integer") (Number :type "Array of Integer") (IsInsertTask :type Boolean))
  (bind (_taskname _index _number _isinserttask) (`parent.GetInsertTask`))
  (return _taskname _index _number _isinserttask))

(fn `Insert Task`
  (params (TaskName :type Name) (Index :type Integer) (Number :type Integer))
  (`parent.Insert Task` TaskName Index Number))

(fn `TaskPlay`
  (returns (isTaskEnd :type Boolean))
  (bind (_end _canselect) (`/Game/Game/MainGame/SugorokuSystem/Props/Pieces/BP_PieceBase.Move` (`self.Piece`)))
  (if _canselect
    (`self.Insert Task` "SelectTile" 0 1))
  (return _end))

(fn `UserConstructionScript`
  (`parent.UserConstructionScript`))