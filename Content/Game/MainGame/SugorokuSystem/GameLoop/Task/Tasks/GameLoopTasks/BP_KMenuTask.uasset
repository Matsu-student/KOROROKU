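; BP_KMenuTask is the menu task in the sugoroku board game's game loop, branching to the next task based on a numeric selection.
; TaskPlay switches on OutputDataNum, returning false for zero, or inserting a dice, map view or card selection task at index 0 and returning true.
; InsertTask only forwards to the parent implementation, and the event graph holds only disabled default events.
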(fn `Insert Task`
  (params (TaskName :type Name) (Index :type Integer) (Number :type Integer))
  (`parent.Insert Task` TaskName Index Number))

(fn `TaskPlay`
  (returns (isTaskEnd :type Boolean))
  (switch `int` (`self.OutputDataNum`)
    (:`0`
      (return false))
    (:`1`
      (`self.Insert Task` "Dice" 0 1)
      (return true))
    (:`2`
      (`self.Insert Task` "ViewMap" 0 1)
      (return true))
    (:`3`
      (`self.Insert Task` "KSelectCard" 0 1)
      (return true))))

(fn `UserConstructionScript`
  (`parent.UserConstructionScript`))