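; Turn counter component for the sugoroku game loop that counts turns upward.
; On BeginPlay it caps the starting turn number at the turn maximum.
; Each Play event calls Count, which increments the turn number without rechecking the maximum and prints it as keyed green debug text.
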(event `self.ReceiveBeginPlay`
  ;[1 1 1] ターンの最大値を超えてないか
  (if (> (`self.TurnNum`) (`self.TurnMax`))
    (set `self.TurnNum` (`self.TurnMax`))))

(event `/Game/Game/MainGame/SugorokuSystem/GameLoop/TurnCounter/BI_TurnCounter.Play`
  (`self.Count`))

(fn `Count`
  (bind _result (`/Engine/EditorBlueprintResources/StandardMacros.IncrementInt` (`self.TurnNum`))
    (:`  `
      (`KismetSystemLibrary.PrintString` (`KismetStringLibrary.Concat_StrStr` (`KismetStringLibrary.Conv_NameToString` (`self.Key`)) "/" (`KismetStringLibrary.Conv_IntToString` _result)) true true (struct :`G` 1.0 :`A` 1.0) 10.0 (`self.Key`)))))