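; Actor component for the sugoroku board game loop that tracks which player's turn it is.
; SwitchPlayer increments a running counter, prints a debug string and returns the next player ID from the PlayerNumber array along with its turn index, wrapping with a hardcoded modulo of four.
; GetNowPlayerNumber indexes that array with the raw counter, without the wrap.
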(fn `GetNowPlayerNumber`
  (returns (NowPlayerNumber :type Integer))
  (return (`|GetArrayItem` (`self.PlayerNumber`) (`self.Counter`))))

(fn `SwitchPlayer`
  (returns (NowPlayerID :type Integer) (PlayerNum :type Integer))
  (bind _returnvalue (mod (`self.Counter`) 4))
  (`/Engine/EditorBlueprintResources/StandardMacros.IncrementInt` (`self.Counter`)
    (:`  `
      (`KismetSystemLibrary.PrintString` (`KismetStringLibrary.Concat_StrStr` (`KismetStringLibrary.Conv_NameToString` (`self.Key`)) "/" (`KismetStringLibrary.Conv_NameToString` "None")) true true (struct :`G` 0.66 :`B` 1.0 :`A` 1.0) 2.0 (`self.Key`))
      (return (`|GetArrayItem` (`self.PlayerNumber`) _returnvalue) _returnvalue))))