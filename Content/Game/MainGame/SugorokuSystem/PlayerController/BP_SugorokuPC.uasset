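; Player controller for the Sugoroku board-game system that relays player input to the current task.
; InputTargetTask stores the task that receives input.
; Keyboard and gamepad actions for decide, cancel and four directions merge into shared Server-prefixed events, unifying both control schemes.
; Each event calls the matching message on the stored task, always passing false, so the task decides what the input means.
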(event `self.ReceiveBeginPlay`)

(event `/Game/Game/MainGame/SugorokuSystem/PlayerController/BI_SetSugorokuPC.InputTargetTask`
  (params (Task :type "Actor Object Reference"))
  ;[1 1 1] 現在のタスクを取得
  (set `self.Task` Task))

(event `EnhancedInput|/Game/Game/Input/Key/IA_KeyDecide`
  (params (ActionValue :type Boolean) (ElapsedSeconds :type "Float (double-precision)") (TriggeredSeconds :type "Float (double-precision)") (InputAction :type "InputAction Object Reference" :default "/Game/Game/Input/Key/IA_KeyDecide.IA_KeyDecide"))
  ;[1 1 1] 操作系の違いを統一した入力を作成しタスクに送信
  (:`Triggered`
    (`self.ServerDecide` :!label _label)))

(event `ServerDecide`
  ;[1 1 1] 操作系の違いを統一した入力を作成しタスクに送信
  (message `/Game/Game/MainGame/SugorokuSystem/PlayerController/BI_SugorokuPC.Decide` (`self.Task`) false))

(event `EnhancedInput|/Game/Game/Input/Pad/IA_PadDecide`
  (params (ActionValue :type Boolean) (ElapsedSeconds :type "Float (double-precision)") (TriggeredSeconds :type "Float (double-precision)") (InputAction :type "InputAction Object Reference" :default "/Game/Game/Input/Pad/IA_PadDecide.IA_PadDecide"))
  ;[1 1 1] 操作系の違いを統一した入力を作成しタスクに送信
  (:`Triggered`
    (goto _label)))

(event `EnhancedInput|/Game/Game/Input/Key/IA_KeyCancel`
  (params (ActionValue :type Boolean) (ElapsedSeconds :type "Float (double-precision)") (TriggeredSeconds :type "Float (double-precision)") (InputAction :type "InputAction Object Reference" :default "/Game/Game/Input/Key/IA_KeyCancel.IA_KeyCancel"))
  ;[1 1 1] 操作系の違いを統一した入力を作成しタスクに送信
  (:`Triggered`
    (`self.ServerCancel` :!label _label_2)))

(event `ServerCancel`
  ;[1 1 1] 操作系の違いを統一した入力を作成しタスクに送信
  (message `/Game/Game/MainGame/SugorokuSystem/PlayerController/BI_SugorokuPC.Cancel` (`self.Task`) false))

(event `EnhancedInput|/Game/Game/Input/Pad/IA_PadCancel`
  (params (ActionValue :type Boolean) (ElapsedSeconds :type "Float (double-precision)") (TriggeredSeconds :type "Float (double-precision)") (InputAction :type "InputAction Object Reference" :default "/Game/Game/Input/Pad/IA_PadCancel.IA_PadCancel"))
  ;[1 1 1] 操作系の違いを統一した入力を作成しタスクに送信
  (:`Triggered`
    (goto _label_2)))

(event `EnhancedInput|/Game/Game/Input/Key/IA_KeyUP`
  (params (ActionValue :type Boolean) (ElapsedSeconds :type "Float (double-precision)") (TriggeredSeconds :type "Float (double-precision)") (InputAction :type "InputAction Object Reference" :default "/Game/Game/Input/Key/IA_KeyUP.IA_KeyUP"))
  ;[1 1 1] 操作系の違いを統一した入力を作成しタスクに送信
  (:`Triggered`
    (`self.ServerUP` :!label _label_3)))

(event `ServerUP`
  ;[1 1 1] 操作系の違いを統一した入力を作成しタスクに送信
  (message `/Game/Game/MainGame/SugorokuSystem/PlayerController/BI_SugorokuPC.UP` (`self.Task`) false))

(event `EnhancedInput|/Game/Game/Input/Pad/IA_PadUP`
  (params (ActionValue :type Boolean) (ElapsedSeconds :type "Float (double-precision)") (TriggeredSeconds :type "Float (double-precision)") (InputAction :type "InputAction Object Reference" :default "/Game/Game/Input/Pad/IA_PadUP.IA_PadUP"))
  ;[1 1 1] 操作系の違いを統一した入力を作成しタスクに送信
  (:`Triggered`
    (goto _label_3)))

(event `EnhancedInput|/Game/Game/Input/Key/IA_KeyDawn`
  (params (ActionValue :type Boolean) (ElapsedSeconds :type "Float (double-precision)") (TriggeredSeconds :type "Float (double-precision)") (InputAction :type "InputAction Object Reference" :default "/Game/Game/Input/Key/IA_KeyDawn.IA_KeyDawn"))
  ;[1 1 1] 操作系の違いを統一した入力を作成しタスクに送信
  (:`Triggered`
    (`self.ServerDawn` :!label _label_4)))

(event `ServerDawn`
  ;[1 1 1] 操作系の違いを統一した入力を作成しタスクに送信
  (message `/Game/Game/MainGame/SugorokuSystem/PlayerController/BI_SugorokuPC.Dawn` (`self.Task`) false))

(event `EnhancedInput|/Game/Game/Input/Pad/IA_PadDawn`
  (params (ActionValue :type Boolean) (ElapsedSeconds :type "Float (double-precision)") (TriggeredSeconds :type "Float (double-precision)") (InputAction :type "InputAction Object Reference" :default "/Game/Game/Input/Pad/IA_PadDawn.IA_PadDawn"))
  ;[1 1 1] 操作系の違いを統一した入力を作成しタスクに送信
  (:`Triggered`
    (goto _label_4)))

(event `EnhancedInput|/Game/Game/Input/Key/IA_KeyLeft`
  (params (ActionValue :type Boolean) (ElapsedSeconds :type "Float (double-precision)") (TriggeredSeconds :type "Float (double-precision)") (InputAction :type "InputAction Object Reference" :default "/Game/Game/Input/Key/IA_KeyLeft.IA_KeyLeft"))
  ;[1 1 1] 操作系の違いを統一した入力を作成しタスクに送信
  (:`Triggered`
    (`self.ServerLeft` :!label _label_5)))

(event `ServerLeft`
  ;[1 1 1] 操作系の違いを統一した入力を作成しタスクに送信
  (message `/Game/Game/MainGame/SugorokuSystem/PlayerController/BI_SugorokuPC.left` (`self.Task`) false))

(event `EnhancedInput|/Game/Game/Input/Pad/IA_PadLeft`
  (params (ActionValue :type Boolean) (ElapsedSeconds :type "Float (double-precision)") (TriggeredSeconds :type "Float (double-precision)") (InputAction :type "InputAction Object Reference" :default "/Game/Game/Input/Pad/IA_PadLeft.IA_PadLeft"))
  ;[1 1 1] 操作系の違いを統一した入力を作成しタスクに送信
  (:`Triggered`
    (goto _label_5)))

(event `EnhancedInput|/Game/Game/Input/Key/IA_KeyRight`
  (params (ActionValue :type Boolean) (ElapsedSeconds :type "Float (double-precision)") (TriggeredSeconds :type "Float (double-precision)") (InputAction :type "InputAction Object Reference" :default "/Game/Game/Input/Key/IA_KeyRight.IA_KeyRight"))
  ;[1 1 1] 操作系の違いを統一した入力を作成しタスクに送信
  (:`Triggered`
    (`self.ServerRight` :!label _label_6)))

(event `ServerRight`
  ;[1 1 1] 操作系の違いを統一した入力を作成しタスクに送信
  (message `/Game/Game/MainGame/SugorokuSystem/PlayerController/BI_SugorokuPC.Right` (`self.Task`) false))

(event `EnhancedInput|/Game/Game/Input/Pad/IA_PadRight`
  (params (ActionValue :type Boolean) (ElapsedSeconds :type "Float (double-precision)") (TriggeredSeconds :type "Float (double-precision)") (InputAction :type "InputAction Object Reference" :default "/Game/Game/Input/Pad/IA_PadRight.IA_PadRight"))
  ;[1 1 1] 操作系の違いを統一した入力を作成しタスクに送信
  (:`Triggered`
    (goto _label_6)))

(fn `UserConstructionScript`)