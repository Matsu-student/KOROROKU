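; Player state for the Sugoroku board game that stores the player's number and current task and drives the main game UI.
; BeginPlay adds the game input mapping context and creates the main UI widget.
; InitMainUI switches the UI to the task's scene, links that scene widget and task to each other, and passes in the player number.
; CliantUpdateMainUI repeats each scene switch, and FinaMainUI resets to scene zero.
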(event `self.ReceiveBeginPlay`
  (`EnhancedInputSubsystemInterface.AddMappingContext` (pcsubsystem `EnhancedInputLocalPlayerSubsystem` (`GameplayStatics.GetPlayerController` 0)) "/Game/Game/Input/IMC_Game.IMC_Game" 0 (struct))
  (bind _returnvalue (`|CreateWidget` "/Game/Game/MainGame/SugorokuSystem/UI/WBP_SugorokuMainUI.WBP_SugorokuMainUI_C"))
  (set `self.MainUI` _returnvalue)
  (`UserWidget.AddToViewport` _returnvalue 0))

(event `/Game/Game/MainGame/SugorokuSystem/PlayerState/BI_SugorokuPS.Set PlayerNumber`
  (params (PlayerNumber :type Integer))
  (set `self.PlayerNumber` PlayerNumber))

(event `/Game/Game/MainGame/SugorokuSystem/PlayerState/BI_SugorokuPS.SetTask`
  (params (NowTask :type "Actor Object Reference"))
  (set `self.Task` NowTask))

(event `/Game/Game/MainGame/SugorokuSystem/PlayerState/BI_SugorokuPS.InitMainUI`
  (bind _sceneid (message `/Game/Game/MainGame/SugorokuSystem/GameLoop/Task/Tasks/TaskBase/BI_Task.GetSceneID` (`self.Task`)))
  (bind _scene (message `/Game/Game/MainGame/SugorokuSystem/UI/BI_SugorokuMainUI.SwichScene` (`self.MainUI`) _sceneid))
  (message `/Game/Game/MainGame/SugorokuSystem/GameLoop/Task/Tasks/TaskBase/BI_Task.SetSceneWidget` (`self.Task`) _scene)
  (message `/Game/Game/MainGame/SugorokuSystem/UI/Scene/BI_Scene.SetTask` _scene (`self.Task`))
  (message `/Game/Game/MainGame/SugorokuSystem/UI/Scene/BI_Scene.SetNowPlayerID` _scene (`self.PlayerNumber`))
  (`self.CliantUpdateMainUI` _sceneid))

(event `/Game/Game/MainGame/SugorokuSystem/PlayerState/BI_SugorokuPS.FinaMainUI`
  (message `/Game/Game/MainGame/SugorokuSystem/UI/BI_SugorokuMainUI.SwichScene` (`self.MainUI`) 0)
  (`self.CliantUpdateMainUI` 0))

(event `CliantUpdateMainUI`
  (params (Index :type Integer))
  (message `/Game/Game/MainGame/SugorokuSystem/UI/BI_SugorokuMainUI.SwichScene` (`self.MainUI`) Index))

(fn `GetPC`
  (returns (PlayerController :type "PlayerController Object Reference"))
  (return (`self.GetPlayerController`)))

(fn `GetPlayerNumber`
  (returns (PlayerNumber :type Integer))
  (return (`self.PlayerNumber`)))

(fn `UserConstructionScript`)