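; BP_ScoreStorage stores player scores for the minigame in a PlayerScore map keyed by integer.
; AddNewStarage registers an entry with a score of zero, using the current map length as its key, and returns that key.
; Tick prints the score under key 0 every frame, and EndPlay clears the map.
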(event `self.ReceiveTick`
  (params (DeltaSeconds :type "Float (single-precision)"))
  (`KismetSystemLibrary.PrintString` (`KismetStringLibrary.Conv_IntToString` (`BlueprintMapLibrary.Map_Find` (`self.PlayerScore`)))))

(event `self.ReceiveEndPlay`
  (params (EndPlayReason :type "EEndPlayReason Enum" :default "Destroyed"))
  (`BlueprintMapLibrary.Map_Clear` (`self.PlayerScore`)))

(fn `Add New Starage`
  (returns (Key :type Integer))
  (locals (ReturnKey :type Integer))
  (bind _output_get (set `local.ReturnKey` (`BlueprintMapLibrary.Map_Length` (`self.PlayerScore`))))
  (`BlueprintMapLibrary.Map_Add` (`self.PlayerScore`) _output_get)
  (return (`local.ReturnKey`)))

(fn `UserConstructionScript`)