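; BP_Timer is a minigame utility that counts calls up to a set end value.
; CountStert sets the CanPlay flag, which lets CountUP increment Counter by one per call until it reaches EndTime, after which CountUP returns true.
; The Blueprint has no active event logic of its own, so counting advances only when CountUP is called, and nothing here resets the counter.
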(fn `CountStert`
  (set `self.CanPlay` true))

(fn `CountUP`
  (returns (End :type Boolean))
  (if (`self.CanPlay`)
    (if (< (`self.Counter`) (`self.EndTime`))
      (`/Engine/EditorBlueprintResources/StandardMacros.IncrementInt` (`self.Counter`))
      (else
        (return true)))))

(fn `UserConstructionScript`)