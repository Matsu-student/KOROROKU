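; BP_MiniGameCH_01 is the Blueprint for minigame 01, apparently its player character, with horizontal movement and a left-click hit.
; Move input passes its 2D vector to the ACConvertToHorizontalMovement component.
; Left mouse sends HitMessage to every actor overlapping its Sphere, excluding itself.
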(event `self.ReceiveBeginPlay`
  (`parent.ReceiveBeginPlay`))

(event `/Game/Game/MiniGame/MiniGamePC/BI_MinGameInput.Move`
  (params (Vector2D :type "Vector2D Structure"))
  (`/Game/Game/MiniGame/Compornent/Movement/AC_ConvertToHorizontalMovement.Move` (`self.AC_ConvertToHorizontalMovement`) Vector2D))

(event `/Game/Game/MiniGame/MiniGamePC/BI_MinGameInput.MouseLeft`
  (bind _overlappingactors (`PrimitiveComponent.GetOverlappingActors` (`self.Sphere`) null))
  (if (`KismetArrayLibrary.Array_IsNotEmpty` _overlappingactors)
    (for _array_element _overlappingactors
      (if (not (== _array_element self))
        (message `/Game/Game/MiniGame/Props/Item/BI_Item.Hit` _array_element)))))

(fn `UserConstructionScript`
  (`parent.UserConstructionScript`))