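; BP_MiniGameGM_01 is the GM Blueprint for mini-game 01, running a timed round with a high-score rule.
; Init initializes BPGameRuleHiScore and starts the count on ACTimer.
; Tick polls the timer's CountUP and, when it returns true, ends the count and has the rule sort the high scores.
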(event `self.ReceiveBeginPlay`)

(event `self.init`
  (`/Game/Game/MiniGame/Compornent/GameRule/Base/AC_GameRuleBase.Init` (`self.BP_GameRuleHiScore`))
  (`/Game/Game/MiniGame/Compornent/Utility/AC_Timer.CountStert` (`self.AC_Timer`)))

(event `self.ReceiveTick`
  (params (DeltaSeconds :type "Float (single-precision)"))
  (bind _end (`/Game/Game/MiniGame/Compornent/Utility/AC_Timer.CountUP` (`self.AC_Timer`)))
  (if _end
    (`/Game/Game/MiniGame/Compornent/Utility/AC_Timer.CountEnd` (`self.AC_Timer`))
    (`/Game/Game/MiniGame/Compornent/GameRule/BP_GameRuleHiScore.HiScoreSort` (`self.BP_GameRuleHiScore`))))

(fn `UserConstructionScript`)