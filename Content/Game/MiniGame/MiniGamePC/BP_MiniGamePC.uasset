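; Player controller for the minigame that relays Enhanced Input to a swappable input target.
; Init adds the IMC_MiniGame mapping context to player 0 and sets the controlled pawn as the default target.
; Move, WASD key and left/right mouse actions are forwarded to the target as message calls, and SetInputTarget can redirect them.
; BeginPlay is empty, and nothing in this graph calls Init.
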(event `self.ReceiveBeginPlay`)

(event `EnhancedInput|/Game/Game/MiniGame/Input/IA_Move`
  (params (ActionValue :type "Vector2D Structure") (ElapsedSeconds :type "Float (double-precision)") (TriggeredSeconds :type "Float (double-precision)") (InputAction :type "InputAction Object Reference" :default "/Game/Game/MiniGame/Input/IA_Move.IA_Move"))
  (:`Triggered`
    (message `/Game/Game/MiniGame/MiniGamePC/BI_MinGameInput.Move` (`self.InputTarget`) ActionValue)))

(event `EnhancedInput|/Game/Game/MiniGame/Input/IA_Key_W`
  (params (ActionValue :type Boolean) (ElapsedSeconds :type "Float (double-precision)") (TriggeredSeconds :type "Float (double-precision)") (InputAction :type "InputAction Object Reference" :default "/Game/Game/MiniGame/Input/IA_Key_W.IA_Key_W"))
  (:`Triggered`
    (message `/Game/Game/MiniGame/MiniGamePC/BI_MinGameInput.Key_W` (`self.InputTarget`))))

(event `EnhancedInput|/Game/Game/MiniGame/Input/IA_Key_S`
  (params (ActionValue :type Boolean) (ElapsedSeconds :type "Float (double-precision)") (TriggeredSeconds :type "Float (double-precision)") (InputAction :type "InputAction Object Reference" :default "/Game/Game/MiniGame/Input/IA_Key_S.IA_Key_S"))
  (:`Triggered`
    (message `/Game/Game/MiniGame/MiniGamePC/BI_MinGameInput.Key_S` (`self.InputTarget`))))

(event `EnhancedInput|/Game/Game/MiniGame/Input/IA_Key_A`
  (params (ActionValue :type Boolean) (ElapsedSeconds :type "Float (double-precision)") (TriggeredSeconds :type "Float (double-precision)") (InputAction :type "InputAction Object Reference" :default "/Game/Game/MiniGame/Input/IA_Key_A.IA_Key_A"))
  (:`Triggered`
    (message `/Game/Game/MiniGame/MiniGamePC/BI_MinGameInput.Key_A` (`self.InputTarget`))))

(event `EnhancedInput|/Game/Game/MiniGame/Input/IA_Key_D`
  (params (ActionValue :type Boolean) (ElapsedSeconds :type "Float (double-precision)") (TriggeredSeconds :type "Float (double-precision)") (InputAction :type "InputAction Object Reference" :default "/Game/Game/MiniGame/Input/IA_Key_D.IA_Key_D"))
  (:`Triggered`
    (message `/Game/Game/MiniGame/MiniGamePC/BI_MinGameInput.Key_D` (`self.InputTarget`))))

(event `EnhancedInput|/Game/Game/MiniGame/Input/IA_MouseLeft`
  (params (ActionValue :type Boolean) (ElapsedSeconds :type "Float (double-precision)") (TriggeredSeconds :type "Float (double-precision)") (InputAction :type "InputAction Object Reference" :default "/Game/Game/MiniGame/Input/IA_MouseLeft.IA_MouseLeft"))
  (:`Triggered`
    (message `/Game/Game/MiniGame/MiniGamePC/BI_MinGameInput.MouseLeft` (`self.InputTarget`))))

(event `EnhancedInput|/Game/Game/MiniGame/Input/IA_MouseRight`
  (params (ActionValue :type Boolean) (ElapsedSeconds :type "Float (double-precision)") (TriggeredSeconds :type "Float (double-precision)") (InputAction :type "InputAction Object Reference" :default "/Game/Game/MiniGame/Input/IA_MouseRight.IA_MouseRight"))
  (:`Triggered`
    (message `/Game/Game/MiniGame/MiniGamePC/BI_MinGameInput.MouseRight` (`self.InputTarget`))))

(fn `Init`
  (`EnhancedInputSubsystemInterface.AddMappingContext` (pcsubsystem `EnhancedInputLocalPlayerSubsystem` (`GameplayStatics.GetPlayerController` 0)) "/Game/Game/MiniGame/Input/IMC_MiniGame.IMC_MiniGame" 0 (struct))
  (`self.SetInputTarget` (`self.K2_GetPawn`)))

(fn `SetInputTarget`
  (params (InputTarget :type "Actor Object Reference"))
  (set `self.InputTarget` InputTarget))

(fn `UserConstructionScript`)