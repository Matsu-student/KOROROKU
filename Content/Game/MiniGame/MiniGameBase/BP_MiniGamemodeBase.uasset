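; BP_MiniGamemodeBase is a minigame game mode base that runs a sequence of timed phases.
; An init event starts the ACTimer component on the current CountList entry, and Tick polls it for completion.
; When a count finishes, it calls CliantSwitchUIIndex on every BP_MiniGamePC to switch UI, resets the timer, and starts the next entry until the list runs out.
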(event `init`
  (`/Game/Game/MiniGame/Compornent/Utility/AC_Timer.CountStert` (`self.AC_Timer`) (`|GetArrayItem` (`self.CountList`) (`self.Count`))))

(event `self.ReceiveTick`
  (params (DeltaSeconds :type "Float (single-precision)"))
  (bind _end (`/Game/Game/MiniGame/Compornent/Utility/AC_Timer.CountUP` (`self.AC_Timer`)))
  (if _end
    (`/Game/Game/MiniGame/Compornent/Utility/AC_Timer.CountEnd` (`self.AC_Timer`))
    (bind _outactors (`GameplayStatics.GetAllActorsOfClass` "/Game/Game/MiniGame/MiniGamePC/BP_MiniGamePC.BP_MiniGamePC_C"))
    (for _array_element _outactors
      (`/Game/Game/MiniGame/MiniGamePC/BP_MiniGamePC.CliantSwitchUIIndex` _array_element))
    (`/Game/Game/MiniGame/Compornent/Utility/AC_Timer.reset` (`self.AC_Timer`))
    (if (< (`self.Count`) (- (`KismetArrayLibrary.Array_Length` (`self.CountList`)) 1))
      (`/Engine/EditorBlueprintResources/StandardMacros.IncrementInt` (`self.Count`)
        (:`  `
          (`/Game/Game/MiniGame/Compornent/Utility/AC_Timer.CountStert` (`self.AC_Timer`) (`|GetArrayItem` (`self.CountList`) (`self.Count`))))))))

(fn `UserConstructionScript`)