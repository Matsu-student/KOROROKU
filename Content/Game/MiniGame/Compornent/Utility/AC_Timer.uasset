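; AC_Timer is a mini-game utility component that works as a frame-counted timer.
; CountStert stores the end time and enables counting unless already running, while CountEnd stops it and Reset also clears the counter.
; CountUP must be called externally, as Tick is unused; each call increments the counter and returns true once it reaches EndTime times 60, so seconds assume 60 calls per second.
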(fn `CountEnd`
  (set `self.CanPlay` false))

(fn `CountStert`
  (params (EndTime :type Integer))
  (if (not (`self.CanPlay`))
    (set `self.EndTime` EndTime)
    (set `self.CanPlay` true)))

(fn `CountUP`
  (returns (End :type Boolean))
  (locals (Compleat :type Boolean :default true))
  (if (`self.CanPlay`)
    (if (< (`self.Counter`) (* (`self.EndTime`) 60))
      (`/Engine/EditorBlueprintResources/StandardMacros.IncrementInt` (`self.Counter`)
        (:`  `
          (return false)))
      (else
        (return true)))
    (else
      (return false))))

(fn `reset`
  (set `self.Counter` 0)
  (set `self.CanPlay` false))