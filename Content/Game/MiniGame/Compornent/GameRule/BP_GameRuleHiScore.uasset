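; BP_GameRuleHiScore is a minigame high-score rule that ranks ScoreStorage's PlayerScore entries from highest to lowest score.
; HiScoreSort copies the scores into Score, then repeatedly moves the maximum into HiScore to build a descending list.
; It then reorders PlayerScore in place by matching each ranked value to entries, searched in reverse, and reinserting them at that rank.
; Neither working array is cleared beforehand, and BeginPlay is unused.
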(fn `HiScoreSort`
  (locals (Insert :type "/Game/Game/MiniGame/ScoreStorage/F_PlayerScore Structure"))
  (bind (_indexofmaxvalue _maxvalue) (`KismetMathLibrary.MaxOfIntArray` (`self.Score`)))
  (`|ExecutionSequence`
    (:`then_0`
      (for _array_element (`/Game/Game/MiniGame/ScoreStorage/BP_ScoreStorage.PlayerScore` (`self.ScoreStorage`))
        (`KismetArrayLibrary.Array_Add` (`self.Score`) (`.Score_5_4E46585A4819AF7E9E6AF484516FD002` (break `/Game/Game/MiniGame/ScoreStorage/F_PlayerScore` _array_element)))))
    (:`then_1`
      (for (_ _array_index) (`/Game/Game/MiniGame/ScoreStorage/BP_ScoreStorage.PlayerScore` (`self.ScoreStorage`))
        (`KismetArrayLibrary.Array_Insert` (`self.HiScore`) _maxvalue _array_index)
        (`KismetArrayLibrary.Array_Remove` (`self.Score`) _indexofmaxvalue)))
    (:`then_2`
      (for (_array_element_2 _array_index_2) (`self.HiScore`)
        (bind (_arrayindex _arrayelement) (`/Engine/EditorBlueprintResources/StandardMacros.ReverseForEachLoop` (`/Game/Game/MiniGame/ScoreStorage/BP_ScoreStorage.PlayerScore` (`self.ScoreStorage`)))
          (:`LoopBody`
            (if (== (`.Score_5_4E46585A4819AF7E9E6AF484516FD002` (break `/Game/Game/MiniGame/ScoreStorage/F_PlayerScore` _arrayelement)) _array_element_2)
              (bind _output_get (set `local.Insert` _arrayelement))
              (`KismetArrayLibrary.Array_Remove` (`/Game/Game/MiniGame/ScoreStorage/BP_ScoreStorage.PlayerScore` (`self.ScoreStorage`)) _arrayindex)
              (`KismetArrayLibrary.Array_Insert` (`/Game/Game/MiniGame/ScoreStorage/BP_ScoreStorage.PlayerScore` (`self.ScoreStorage`)) _output_get _array_index_2)))))
      (return))))