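; BP_CardSlot is a card-layout actor for the card game that arranges debug cards along a spline.
; On BeginPlay it spawns ten BP_DebugCard actors, stores them in Cards, and spaces them evenly by spline distance, ending at the spline's far end.
; Each card takes the spline's world location and uses the negated spline pitch as its roll.
; SetCard and the construction script are empty.
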(event `self.ReceiveBeginPlay`
  (bind _cards (`self.Cards`))
  (bind _spline (`self.Spline`))
  (for _ (range 10)
    (bind _returnvalue (`|SpawnActorFromClass` "/Game/Game/GameMain/CardGameSystem/Card/Cards/BP_DebugCard.BP_DebugCard_C" (`KismetMathLibrary.MakeTransform` (0.0 0.0 0.0)) "Undefined" "MultiplyWithRoot" null null))
    (`KismetArrayLibrary.Array_Add` (`self.Cards`) _returnvalue))
  (for (_array_element _array_index) _cards
    (bind _returnvalue_2 (* (`SplineComponent.GetSplineLength` _spline) (* (`KismetMathLibrary.Conv_IntToDouble` (+ _array_index 1)) (/ 1.0 (`KismetMathLibrary.Conv_IntToDouble` (`KismetArrayLibrary.Array_Length` _cards))))))
    (bind (_returnvalue_x _returnvalue_y _returnvalue_z) (`KismetMathLibrary.BreakVector` (`SplineComponent.GetLocationAtDistanceAlongSpline` _spline _returnvalue_2 "World")))
    (`self.K2_SetActorLocation` _array_element (`KismetMathLibrary.MakeVector` _returnvalue_x _returnvalue_y _returnvalue_z) false false)
    (bind (_returnvalue_roll _returnvalue_pitch) (`KismetMathLibrary.BreakRotator` (`SplineComponent.GetRotationAtDistanceAlongSpline` _spline _returnvalue_2 "World")))
    (`self.K2_SetActorRotation` _array_element (`KismetMathLibrary.MakeRotator` (* _returnvalue_pitch -1.0)) false)))

(fn `SetCard`)

(fn `UserConstructionScript`)