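; BP_TaskBase is the base task for the Sugoroku game loop, with overridable init, play and finish steps; the default TaskPlay logs and returns true.
; It receives the player ID, controller, card system and scene widget, driving the widget's init/finish and forwarding directional, decide and cancel input when valid.
; It also records follow-up task insertion requests and provides frame-count Wait and call-count Once helpers.
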(event `/Game/Game/GameMain/SugorokuSystem/GameLoop/Task/Tasks/TaskBase/BI_Task.SetNowPlayerID`
  (params (PlayerID :type Integer))
  (set `self.NowPlayerID` PlayerID))

(event `/Game/Game/GameMain/SugorokuSystem/GameLoop/Task/Tasks/TaskBase/BI_Task.TaskInit`
  (`/Game/Game/GameMain/SugorokuSystem/UI/Scene/SceneBase/WBP_SceneBase.SceneInit` (`self.Scene Widget`)))

(event `/Game/Game/GameMain/SugorokuSystem/GameLoop/Task/Tasks/TaskBase/BI_Task.SetSceneWidget`
  (params (SceneWidget :type "/Game/Game/GameMain/SugorokuSystem/UI/Scene/SceneBase/WBP_SceneBase Object Reference"))
  (set `self.Scene Widget` SceneWidget))

(event `/Game/Game/GameMain/SugorokuSystem/GameLoop/Task/Tasks/TaskBase/BI_Task.TaskFina`
  (`/Game/Game/GameMain/SugorokuSystem/UI/Scene/SceneBase/WBP_SceneBase.SceneFina` (`self.Scene Widget`)))

(event `/Game/Game/GameMain/SugorokuSystem/Input/BI_SugorokuPC.SetPlayerContller`
  (params (PlayerContller :type "PlayerController Object Reference"))
  (set `self.Player Contller` PlayerContller))

(event `/Game/Game/GameMain/SugorokuSystem/GameLoop/Task/Tasks/TaskBase/BI_Task.SetCardGameSytem`
  (params (CardGameSystem :type "ActorComponent Object Reference"))
  (set `self.Card Game System` CardGameSystem))

(event `/Game/Game/GameMain/SugorokuSystem/GameLoop/Task/Tasks/TaskBase/BI_Task.GetOutputDataNum`
  (params (DataNum :type Integer))
  (set `self.OutputDataNum` DataNum))

(event `/Game/Game/GameMain/SugorokuSystem/Input/BI_SugorokuPC.UP`
  (params (Input :type Boolean))
  (bind _canuse (`self.CanUseScene`))
  (if _canuse
    (message `/Game/Game/GameMain/SugorokuSystem/UI/Scene/BI_Scene.UIUP` (`self.Scene Widget`))))

(event `/Game/Game/GameMain/SugorokuSystem/Input/BI_SugorokuPC.Dawn`
  (params (Input :type Boolean))
  (bind _canuse (`self.CanUseScene`))
  (if _canuse
    (message `/Game/Game/GameMain/SugorokuSystem/UI/Scene/BI_Scene.UIDawn` (`self.Scene Widget`))))

(event `/Game/Game/GameMain/SugorokuSystem/Input/BI_SugorokuPC.left`
  (params (Input :type Boolean))
  (bind _canuse (`self.CanUseScene`))
  (if _canuse
    (message `/Game/Game/GameMain/SugorokuSystem/UI/Scene/BI_Scene.UILeft` (`self.Scene Widget`))))

(event `/Game/Game/GameMain/SugorokuSystem/Input/BI_SugorokuPC.Right`
  (params (Input :type Boolean))
  (bind _canuse (`self.CanUseScene`))
  (if _canuse
    (message `/Game/Game/GameMain/SugorokuSystem/UI/Scene/BI_Scene.UIRight` (`self.Scene Widget`))))

(event `/Game/Game/GameMain/SugorokuSystem/Input/BI_SugorokuPC.Decide`
  (params (Input :type Boolean))
  (bind _canuse (`self.CanUseScene`))
  (if _canuse
    (message `/Game/Game/GameMain/SugorokuSystem/UI/Scene/BI_Scene.UIDecide` (`self.Scene Widget`))))

(event `/Game/Game/GameMain/SugorokuSystem/Input/BI_SugorokuPC.Cancel`
  (params (Input :type Boolean))
  (bind _canuse (`self.CanUseScene`))
  (if _canuse
    (message `/Game/Game/GameMain/SugorokuSystem/UI/Scene/BI_Scene.UICancel` (`self.Scene Widget`))))

(fn `CanUseScene`
  (returns (CanUse :type Boolean))
  (return (!= (`self.Scene Widget`) null)))

(fn `GetInsertTask`
  (returns (TaskName :type "Array of Name") (Index :type "Array of Integer") (Number :type "Array of Integer") (IsInsertTask :type Boolean))
  (return (`self.InsertTaskName`) (`self.InsertIndex`) (`self.Number`) (`self.IsInsertTask`)))

(fn `GetSceneID`
  (returns (SceneID :type Integer))
  (return (`self.ViewSceneID`)))

(fn `Insert Task`
  (params (TaskName :type Name) (Index :type Integer) (Number :type Integer))
  (`KismetArrayLibrary.Array_Add` (`self.InsertTaskName`) TaskName)
  (`KismetArrayLibrary.Array_Add` (`self.InsertIndex`) Index)
  (`KismetArrayLibrary.Array_Add` (`self.Number`) Number)
  (if (not (`self.IsInsertTask`))
    (set `self.IsInsertTask` true))
  (return))

(fn `Once`
  (returns (IsUse :type Boolean))
  (locals (over :type Boolean :default false))
  (set `local.over` (> (`self.countUse`) 0))
  (`/Engine/EditorBlueprintResources/StandardMacros.IncrementInt` (`self.countUse`)
    (:`  `
      (return (`local.over`)))))

(fn `TaskPlay`
  (returns (isTaskEnd :type Boolean))
  (`KismetSystemLibrary.PrintString` (`KismetStringLibrary.Concat_StrStr` (`KismetStringLibrary.Conv_NameToString` (`self.Key`)) "/" "Play") true true (struct :`G` 0.66 :`B` 1.0 :`A` 1.0) 10.0 (`self.Key`))
  (return true))

(fn `UserConstructionScript`)

(fn `Wait`
  (params (Frame :type Integer))
  (returns (End :type Boolean))
  (bind _result (`/Engine/EditorBlueprintResources/StandardMacros.IncrementInt` (`self.CountFrame`))
    (:`  `
      (`KismetSystemLibrary.PrintString` (`KismetStringLibrary.Conv_IntToString` _result) true true (struct :`R` 1.0 :`B` 0.419177 :`A` 1.0) 2.0 "WaitTimer")
      (if (>= (`self.CountFrame`) Frame)
        (set `self.CountFrame` 0)
        (return true)
        (else
          (return false))))))