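; BP_CardDrawTask is a task in the sugoroku board game loop that runs the card-draw tile effect.
; On BeginPlay it caches the AC_CardGameSystem component found on the BP_SugorokuSystem actor.
; TaskPlay uses the parent's Once guard to order the card-draw message, then returns whether that message order has ended, signalling task completion.
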(event `self.ReceiveBeginPlay`
  (`parent.ReceiveBeginPlay`)
  (bind _returnvalue (`GameplayStatics.GetActorOfClass` "/Game/Game/GameMain/SugorokuSystem/BP_SugorokuSystem.BP_SugorokuSystem_C"))
  (for _array_element (`self.K2_GetComponentsByClass` _returnvalue "/Game/Game/GameMain/SugorokuSystem/CardGameSystem/AC_CardGameSystem.AC_CardGameSystem_C")
    (set `self.CardGameSystem` _array_element)))

(fn `Once`
  (returns (IsUse :type Boolean))
  (bind _isuse (`parent.Once`))
  (return _isuse))

(fn `TaskPlay`
  (returns (isTaskEnd :type Boolean))
  (bind _isuse (`self.Once`))
  (if (not _isuse)
    (message `/Game/Game/GameMain/SugorokuSystem/CardGameSystem/BI_CardGameSystem.OrderDrawCard` (`self.CardGameSystem`)))
  (bind _isendorder (message `/Game/Game/GameMain/SugorokuSystem/CardGameSystem/BI_CardGameSystem.GetIsEndOrder` (`self.CardGameSystem`)))
  (return _isendorder))

(fn `UserConstructionScript`
  (`parent.UserConstructionScript`))