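; Game-loop task for the sugoroku board game that moves the current player's piece.
; On BeginPlay it caches every BP_PieceBase actor in the level.
; TaskPlay finds the piece matching NowPlayerID, calls InitMove and Move on it, and returns the move's End result as the task result.
; When Move reports CanSelect, it inserts a SelectTile task at the head index through the parent's task-insertion logic.
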(event `self.ReceiveBeginPlay`
  (`parent.ReceiveBeginPlay`)
  (bind _outactors (`GameplayStatics.GetAllActorsOfClass` "/Game/Game/GameMain/SugorokuSystem/Props/Pieces/BP_PieceBase.BP_PieceBase_C"))
  (set `self.Piece` _outactors))

(fn `GetInsertTask`
  (returns (TaskName :type "Array of Name") (Index :type "Array of Integer") (Number :type "Array of Integer") (IsInsertTask :type Boolean))
  (bind (_taskname _index _number _isinserttask) (`parent.GetInsertTask`))
  (return _taskname _index _number _isinserttask))

(fn `Insert Task`
  (params (TaskName :type Name) (Index :type Integer) (Number :type Integer))
  (`parent.Insert Task` TaskName Index Number))

(fn `TaskPlay`
  (returns (isTaskEnd :type Boolean))
  (for _array_element (`self.Piece`)
    (if (== (`/Game/Game/GameMain/SugorokuSystem/Props/Pieces/BP_PieceBase.PlayerID` _array_element) (`self.NowPlayerID`))
      (`/Game/Game/GameMain/SugorokuSystem/Props/Pieces/BP_PieceBase.InitMove` _array_element)
      (bind (_end _canselect) (`/Game/Game/GameMain/SugorokuSystem/Props/Pieces/BP_PieceBase.Move` _array_element))
      (break)))
  (if _canselect
    (`self.Insert Task` "SelectTile" 0 1))
  (return _end))

(fn `UserConstructionScript`
  (`parent.UserConstructionScript`))