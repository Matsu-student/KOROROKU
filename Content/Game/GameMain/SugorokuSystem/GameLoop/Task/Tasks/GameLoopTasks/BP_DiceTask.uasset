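; Game-loop task that runs the dice roll in the sugoroku board game.
; On init it spawns a dice scene actor and finds the die, which TaskPlay keeps rolling until Decide input arrives.
; It then stops the die through a Once gate, waits briefly, destroys it and inserts a Move task carrying the rolled number.
; The scene actor is destroyed when the task finishes.
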(event `self.ReceiveBeginPlay`
  (`parent.ReceiveBeginPlay`))

(event `/Game/Game/GameMain/SugorokuSystem/GameLoop/Task/Tasks/TaskBase/BI_Task.TaskInit`
  (bind _returnvalue (`|SpawnActorFromClass` "/Game/Game/GameMain/SugorokuSystem/UI/Scene/DiceScene/BP_DiceSceneActor.BP_DiceSceneActor_C" (`KismetMathLibrary.MakeTransform` (1000.0 0.0 0.0)) "Undefined" "MultiplyWithRoot" null null))
  (set `self.DiceScene` _returnvalue)
  (bind _returnvalue_2 (`GameplayStatics.GetActorOfClass` "/Game/Game/GameMain/SugorokuSystem/Props/Dice/BP_Dice.BP_Dice_C"))
  (set `self.Dice` _returnvalue_2))

(event `/Game/Game/GameMain/SugorokuSystem/GameLoop/Task/Tasks/TaskBase/BI_Task.TaskFina`
  (`self.K2_DestroyActor` (`self.DiceScene`)))

(event `/Game/Game/GameMain/SugorokuSystem/Input/BI_SugorokuPC.Decide`
  (params (Input :type Boolean))
  (set `self.IsPush` Input))

(fn `GetInsertTask`
  (returns (TaskName :type "Array of Name") (Index :type "Array of Integer") (Number :type "Array of Integer") (IsInsertTask :type Boolean))
  (bind (_taskname _index _number _isinserttask) (`parent.GetInsertTask`))
  (return _taskname _index _number _isinserttask))

(fn `GetSceneID`
  (returns (SceneID :type Integer))
  (bind _sceneid (`parent.GetSceneID`))
  (return _sceneid))

(fn `Insert Task`
  (params (TaskName :type Name) (Index :type Integer) (Number :type Integer))
  (`parent.Insert Task` TaskName Index Number))

(fn `Once`
  (returns (IsUse :type Boolean))
  (bind _isuse (`parent.Once`))
  (return _isuse))

(fn `TaskPlay`
  (returns (isTaskEnd :type Boolean))
  (if (`self.IsPush`)
    (bind _isuse (`self.Once`))
    (if _isuse
      (bind _end (`self.Wait` 100))
      (if _end
        (`self.K2_DestroyActor` (`self.Dice`))
        (`self.Insert Task` "Move" 0 (`self.DiceNumber`))
        (return true)
        (else
          (return false)))
      (else
        (bind _number (`/Game/Game/GameMain/SugorokuSystem/Props/Dice/BP_Dice.StopRoll` (`self.Dice`)))
        (set `self.DiceNumber` _number)
        (return false)))
    (else
      (`/Game/Game/GameMain/SugorokuSystem/Props/Dice/BP_Dice.Start Roll` (`self.Dice`))
      (return false))))

(fn `UserConstructionScript`
  (`parent.UserConstructionScript`))

(fn `Wait`
  (params (Frame :type Integer))
  (returns (End :type Boolean))
  (bind _end (`parent.Wait` Frame))
  (return _end))