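; BP_SelectCardTask is a game-loop task for the card selection step of the sugoroku board game.
; On init it switches input to Game and UI, then messages the CardGameSystem to draw a hand, show it and start selection.
; TaskPlay reports whether OutputDataNum is non-zero, and finalization restores game-only input.
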(event `/Game/Game/GameMain/SugorokuSystem/GameLoop/Task/Tasks/TaskBase/BI_Task.TaskInit`
  (`WidgetBlueprintLibrary.SetInputMode_GameAndUIEx` (`self.Player Contller`) null "DoNotLock" true true)
  (for _ (range 5)
    (message `/Game/Game/GameMain/SugorokuSystem/CardGameSystem/BI_CardGameSystem.OrderDrawCard` (`self.Card Game System`)))
  (message `/Game/Game/GameMain/SugorokuSystem/CardGameSystem/BI_CardGameSystem.OrderViewCards` (`self.Card Game System`))
  (message `/Game/Game/GameMain/SugorokuSystem/CardGameSystem/BI_CardGameSystem.OrderInitCardSelect` (`self.Card Game System`)))

(event `/Game/Game/GameMain/SugorokuSystem/GameLoop/Task/Tasks/TaskBase/BI_Task.TaskFina`
  (`WidgetBlueprintLibrary.SetInputMode_GameOnly` (`self.Player Contller`)))

(event `/Game/Game/GameMain/SugorokuSystem/GameLoop/Task/Tasks/TaskBase/BI_Task.SetSceneWidget`
  (params (SceneWidget :type "/Game/Game/GameMain/SugorokuSystem/UI/Scene/SceneBase/WBP_SceneBase Object Reference"))
  (set `self.Scene Widget` SceneWidget))

(fn `GetSceneID`
  (returns (SceneID :type Integer))
  (bind _sceneid (`parent.GetSceneID`))
  (return _sceneid))

(fn `Insert Task`
  (params (TaskName :type Name) (Index :type Integer) (Number :type Integer))
  (`parent.Insert Task` TaskName Index Number))

(fn `TaskPlay`
  (returns (isTaskEnd :type Boolean))
  (return (!= (`self.OutputDataNum`) 0)))

(fn `UserConstructionScript`
  (`parent.UserConstructionScript`))

(fn `Wait`
  (params (Frame :type Integer))
  (returns (End :type Boolean))
  (bind _end (`parent.Wait` Frame))
  (return _end))