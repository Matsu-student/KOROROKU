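; BP_ViewMap is a sugoroku game-loop task that lets the current player look around the map.
; On init it finds that player's piece, spawns a BP_MapCamera at its transform and switches to it through AC_CameraSwitcher.
; Directional events drive both the scene widget and the camera, and a non-zero OutputDataNum inserts the SMenu task.
; On finish it switches the view back to the piece and destroys the camera.
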(event `/Game/Game/GameMain/SugorokuSystem/GameLoop/Task/Tasks/TaskBase/BI_Task.TaskInit`
  (bind _outactors (`GameplayStatics.GetAllActorsOfClass` "/Game/Game/GameMain/SugorokuSystem/Props/Pieces/BP_PieceBase.BP_PieceBase_C"))
  (for _array_element _outactors
    (if (== (`/Game/Game/GameMain/SugorokuSystem/Props/Pieces/BP_PieceBase.PlayerID` _array_element) (`self.NowPlayerID`))
      (bind _output_get (set `self.ViewTaget` _array_element))
      (bind _returnvalue (`|SpawnActorFromClass` "/Game/Game/GameMain/SugorokuSystem/Props/Camera/BP_MapCamera.BP_MapCamera_C" (`self.GetTransform` _output_get) "Undefined" "MultiplyWithRoot" null null))
      (set `self.MapCamera` _returnvalue)
      (break)))
  (bind _returnvalue_2 (`GameplayStatics.GetActorOfClass` "/Game/Game/GameMain/SugorokuSystem/BP_SugorokuSystem.BP_SugorokuSystem_C"))
  (set `self.CameraSwitcher` (`self.GetComponentByClass` _returnvalue_2 "/Game/Game/GameMain/SugorokuSystem/GameLoop/CameraSwitcher/AC_CameraSwitcher.AC_CameraSwitcher_C"))
  (`/Game/Game/GameMain/SugorokuSystem/GameLoop/CameraSwitcher/AC_CameraSwitcher.SwitchCamera` (`self.CameraSwitcher`) (`self.MapCamera`)))

(event `/Game/Game/GameMain/SugorokuSystem/GameLoop/Task/Tasks/TaskBase/BI_Task.TaskFina`
  (`/Game/Game/GameMain/SugorokuSystem/GameLoop/CameraSwitcher/AC_CameraSwitcher.SwitchCamera` (`self.CameraSwitcher`) (`self.ViewTaget`))
  (`self.K2_DestroyActor` (`self.MapCamera`)))

(event `/Game/Game/GameMain/SugorokuSystem/Input/BI_SugorokuPC.UP`
  (params (Input :type Boolean))
  (message `/Game/Game/GameMain/SugorokuSystem/UI/Scene/BI_Scene.UIUP` (`self.Scene Widget`))
  (`/Game/Game/GameMain/SugorokuSystem/Props/Camera/BP_MapCamera.UP` (`self.MapCamera`)))

(event `/Game/Game/GameMain/SugorokuSystem/Input/BI_SugorokuPC.Dawn`
  (params (Input :type Boolean))
  (message `/Game/Game/GameMain/SugorokuSystem/UI/Scene/BI_Scene.UIDawn` (`self.Scene Widget`))
  (`/Game/Game/GameMain/SugorokuSystem/Props/Camera/BP_MapCamera.Dawn` (`self.MapCamera`)))

(event `/Game/Game/GameMain/SugorokuSystem/Input/BI_SugorokuPC.left`
  (params (Input :type Boolean))
  (message `/Game/Game/GameMain/SugorokuSystem/UI/Scene/BI_Scene.UILeft` (`self.Scene Widget`))
  (`/Game/Game/GameMain/SugorokuSystem/Props/Camera/BP_MapCamera.Left` (`self.MapCamera`)))

(event `/Game/Game/GameMain/SugorokuSystem/Input/BI_SugorokuPC.Right`
  (params (Input :type Boolean))
  (message `/Game/Game/GameMain/SugorokuSystem/UI/Scene/BI_Scene.UIRight` (`self.Scene Widget`))
  (`/Game/Game/GameMain/SugorokuSystem/Props/Camera/BP_MapCamera.Rigft` (`self.MapCamera`)))

(fn `Insert Task`
  (params (TaskName :type Name) (Index :type Integer) (Number :type Integer))
  (`parent.Insert Task` TaskName Index Number))

(fn `TaskPlay`
  (returns (isTaskEnd :type Boolean))
  (if (!= (`self.OutputDataNum`) 0)
    (`self.Insert Task` "SMenu" 0 1)
    (return true)))

(fn `UserConstructionScript`
  (`parent.UserConstructionScript`))