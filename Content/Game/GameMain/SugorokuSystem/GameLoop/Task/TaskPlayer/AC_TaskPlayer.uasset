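; Task-queue component for the sugoroku board game that runs named tasks one at a time for the current player.
; Process merges pending additions and inserts, then spawns the next task's actor class from DT_TaskRegistration and links it to the player controller, UI scene and card system.
; It polls the task, accepts its inserts, destroys it when finished and returns true after BP_EndTask.
; Queued deletions loop over AddTask, not DelTask.
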(event `self.ReceiveBeginPlay`
  (bind _outactors (`GameplayStatics.GetAllActorsOfClass` "/Game/Game/GameMain/SugorokuSystem/Input/BP_SugorokuPC.BP_SugorokuPC_C"))
  (set `self.PlayerControllers` _outactors)
  (bind _foundwidgets (`WidgetBlueprintLibrary.GetAllWidgetsOfClass` "/Game/Game/GameMain/SugorokuSystem/UI/WBP_SugorokuMainUI.WBP_SugorokuMainUI_C"))
  (for _array_element _foundwidgets
    (set `self.SugorokuMainUI` _array_element)
    (bind _returnvalue (`GameplayStatics.GetActorOfClass` "/Game/Game/GameMain/SugorokuSystem/BP_SugorokuSystem.BP_SugorokuSystem_C"))
    (set `self.CardGameSystem` (`Actor.GetComponentByClass` _returnvalue "/Game/Game/GameMain/SugorokuSystem/CardGameSystem/AC_CardGameSystem.AC_CardGameSystem_C"))))

(event `/Game/Game/GameMain/SugorokuSystem/GameLoop/Task/TaskPlayer/BI_TaskPlayer.OrderAdd`
  (params (TaskName :type Name))
  (`self.Add` TaskName))

(event `/Game/Game/GameMain/SugorokuSystem/GameLoop/Task/TaskPlayer/BI_TaskPlayer.OrderInsert`
  (params (InsertTask :type Name) (InsertIndex :type Integer) (TaskNum :type Integer))
  (`self.Insert` InsertTask InsertIndex TaskNum))

(event `/Game/Game/GameMain/SugorokuSystem/GameLoop/Task/TaskPlayer/BI_TaskPlayer.OrderDel`
  (params (TaskName :type Name))
  (`self.Del` TaskName))

(fn `Add`
  (params (NewTask :type "Name (by ref)"))
  (`KismetArrayLibrary.Array_Add` (`self.AddTask`) NewTask))

(fn `ClassSerch`
  (params (Task :type Name))
  (returns (TaskClass :type "/Game/Game/GameMain/SugorokuSystem/GameLoop/Task/Tasks/TaskBase/BP_TaskBase Class Reference"))
  (bind _outrownames (`DataTableFunctionLibrary.GetDataTableRowNames` "/Game/Game/GameMain/SugorokuSystem/GameLoop/Task/Tasks/Registration/DT_TaskRegistration.DT_TaskRegistration"))
  (for _array_element _outrownames
    (bind _returnvalue (`|GetDataTableRow` "/Game/Game/GameMain/SugorokuSystem/GameLoop/Task/Tasks/Registration/DT_TaskRegistration.DT_TaskRegistration" _array_element)
      (:`then`
        (bind (_taskname _taskclass) (break `/Game/Game/GameMain/SugorokuSystem/GameLoop/Task/Tasks/Registration/F_TaskSearchData` _returnvalue))
        (if (== Task _taskname)
          (return _taskclass))))))

(fn `Del`
  (params (DelTask :type "Name (by ref)"))
  (`KismetArrayLibrary.Array_Add` (`self.DelTask`) DelTask))

(fn `Insert`
  (params (TaskName :type Name) (InsertIndex :type Integer) (TaskNum :type Integer))
  (`KismetArrayLibrary.Array_Add` (`self.InsertTask`) TaskName)
  (`KismetArrayLibrary.Array_Add` (`self.Insert Index`) InsertIndex)
  (`KismetArrayLibrary.Array_Add` (`self.Task Num`) TaskNum)
  (set `self.Is Insert Task` false))

(fn `InsertTasks`
  (params (TaskName :type "Array of Name (by ref)") (Index :type "Array of Integer") (TaskNum :type "Array of Integer"))
  (if (`self.Is Insert Task`)
    (for (_array_element _array_index) TaskName
      (for _ (range (`|GetArrayItem` TaskNum _array_index))
        (`KismetArrayLibrary.Array_Insert` (`self.Tasks`) _array_element (`|GetArrayItem` Index _array_index))))
    (`KismetArrayLibrary.Array_Clear` (`self.InsertTask`))
    (`KismetArrayLibrary.Array_Clear` (`self.Insert Index`))
    (`KismetArrayLibrary.Array_Clear` (`self.Task Num`))
    (set `self.Is Insert Task` false)
    (return)))

(fn `Process`
  (params (NowPlayerID :type Integer))
  (returns (isEndPlay :type Boolean))
  (locals (ControllerID :type Integer :default 0) (PlayerID :type Integer))
  (bind _addtask (`self.AddTask`))
  (bind _addtask_2 (`self.AddTask`))
  (set `local.PlayerID` NowPlayerID)
  (if (> (`KismetArrayLibrary.Array_Length` (`self.AddTask`)) 0)
    (for _array_element _addtask_2
      (`KismetArrayLibrary.Array_Add` (`self.Tasks`) _array_element))
    (`KismetArrayLibrary.Array_Clear` _addtask_2))
  (`self.InsertTasks` (`self.InsertTask`) (`self.Insert Index`) (`self.Task Num`))
  (if (`self.isPlay`) :!label _label
    (bind _istaskend (message `/Game/Game/GameMain/SugorokuSystem/GameLoop/Task/Tasks/TaskBase/BI_Task.TaskPlay` (`self.Task`)))
    (bind (_taskname _index _number _isinserttask) (message `/Game/Game/GameMain/SugorokuSystem/GameLoop/Task/Tasks/TaskBase/BI_Task.GetInsertTask` (`self.Task`)))
    (set `self.Is Insert Task` _isinserttask)
    (`self.InsertTasks` _taskname _index _number)
    (if _istaskend
      (if (== (`GameplayStatics.GetObjectClass` (`self.Task`)) "/Game/Game/GameMain/SugorokuSystem/GameLoop/Task/Tasks/GameLoopTasks/BP_EndTask.BP_EndTask_C")
        (set `self.isEndPlay` true)
        (else
          (set `self.isEndPlay` false)))
      (message `/Game/Game/GameMain/SugorokuSystem/GameLoop/Task/Tasks/TaskBase/BI_Task.TaskFina` (`self.Task`))
      (`Actor.K2_DestroyActor` (`self.Task`))
      (message `/Game/Game/GameMain/SugorokuSystem/Input/BI_SetSugorokuPC.InputTargetTask` (`self.PlayerController`) null)
      (set `self.isPlay` false)
      (if (> (`KismetArrayLibrary.Array_Length` (`self.DelTask`)) 0)
        (for _array_element_2 _addtask
          (for (_array_element_3 _array_index) (`self.Tasks`)
            (if (== _array_element_3 _array_element_2)
              (`KismetArrayLibrary.Array_Remove` (`self.Tasks`) _array_index)
              (break))))
        (`KismetArrayLibrary.Array_Clear` _addtask))
      (return (`self.isEndPlay`))
      (else
        (bind _output_get (set `self.isEndPlay` false))
        (return _output_get)))
    (else
      (bind _output_get_2 (set `self.ProcessTask` (`|GetArrayItem` (`self.Tasks`)))) ; タスク名からタスク割り出し処理を書く
      (bind _taskclass (`self.ClassSerch` _output_get_2))
      (bind _returnvalue (`|SpawnActorFromClass` _taskclass (`KismetMathLibrary.MakeTransform` (0.0 0.0 0.0)) "Undefined" "MultiplyWithRoot" null null))
      (set `self.Task` _returnvalue)
      (bind _output_get_3 (set `self.PlayerController` (`|GetArrayItem` (`self.PlayerControllers`) (`local.PlayerID`))))
      (message `/Game/Game/GameMain/SugorokuSystem/Input/BI_SetSugorokuPC.InputTargetTask` _output_get_3 (`self.Task`))
      (message `/Game/Game/GameMain/SugorokuSystem/Input/BI_SugorokuPC.SetPlayerContller` (`self.Task`) _output_get_3)
      (message `/Game/Game/GameMain/SugorokuSystem/GameLoop/Task/Tasks/TaskBase/BI_Task.SetNowPlayerID` (`self.Task`) (`local.PlayerID`))
      (bind _sceneid (message `/Game/Game/GameMain/SugorokuSystem/GameLoop/Task/Tasks/TaskBase/BI_Task.GetSceneID` (`self.Task`)))
      (bind _returnvalue_2 (`/Game/Game/GameMain/SugorokuSystem/UI/WBP_SugorokuMainUI.SwitchScene` (`self.SugorokuMainUI`) _sceneid))
      (message `/Game/Game/GameMain/SugorokuSystem/GameLoop/Task/Tasks/TaskBase/BI_Task.SetSceneWidget` (`self.Task`) _returnvalue_2)
      (message `/Game/Game/GameMain/SugorokuSystem/UI/Scene/BI_Scene.SetTask` _returnvalue_2 (`self.Task`))
      (message `/Game/Game/GameMain/SugorokuSystem/UI/Scene/BI_Scene.SetNowPlayerID` _returnvalue_2 (`local.PlayerID`))
      (message `/Game/Game/GameMain/SugorokuSystem/GameLoop/Task/Tasks/TaskBase/BI_Task.SetCardGameSytem` (`self.Task`) (`self.CardGameSystem`))
      (if (> (`KismetArrayLibrary.Array_Length` (`self.Tasks`)) 0)
        (`KismetArrayLibrary.Array_Remove` (`self.Tasks`)))
      (set `self.isPlay` true)
      (message `/Game/Game/GameMain/SugorokuSystem/GameLoop/Task/Tasks/TaskBase/BI_Task.TaskInit` (`self.Task`)) ; 初期化
      (goto _label))))