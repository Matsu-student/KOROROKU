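; Actor component for the Sugoroku game loop that switches the players' camera to a given view target.
; On BeginPlay it caches all BP_SugorokuPC actors in the level.
; SwitchCamera calls SetViewTargetWithBlend for each cached controller when online, fetched by array index through GetPlayerController, and only for player 0 otherwise.
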(event `self.ReceiveBeginPlay`
  (bind _outactors (`GameplayStatics.GetAllActorsOfClass` "/Game/Game/GameMain/SugorokuSystem/Input/BP_SugorokuPC.BP_SugorokuPC_C"))
  (set `self.SugorokuPCs` _outactors))

(fn `SwitchCamera`
  (params (NewViewTarget :type "Actor Object Reference"))
  (if (`self.IsOnline`)
    (for (_ _array_index) (`self.SugorokuPCs`)
      (`PlayerController.SetViewTargetWithBlend` (`GameplayStatics.GetPlayerController` _array_index) NewViewTarget 0.0 "VTBlend_Linear" 0.0 false))
    (else
      (`PlayerController.SetViewTargetWithBlend` (`GameplayStatics.GetPlayerController` 0) NewViewTarget 0.0 "VTBlend_Linear" 0.0 false))))