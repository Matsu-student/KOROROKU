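; BP_DiceTask is a game-loop task for the sugoroku board game that rolls a die until the player presses the decision input.
; BeginPlay spawns a BP_SugorokuDice at a fixed location, and IA_Decision sets a PushButton flag.
; Each Play call starts the roll, then, if the flag is set, stops the roll, destroys the die and returns true.
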(event `self.ReceiveBeginPlay`
  (`parent.ReceiveBeginPlay`)
  (bind _returnvalue (`|SpawnActorFromClass` "/Game/Game/GameMain/SugorokuSystem/Dice/BP_SugorokuDice.BP_SugorokuDice_C" (`KismetMathLibrary.MakeTransform` (500.0 0.0 100.0)) "Undefined" "MultiplyWithRoot" null null))
  (set `self.Dice` _returnvalue))

(event `EnhancedInput|/Game/Game/GameMain/Input/IA_Decision`
  (params (ActionValue :type Boolean) (ElapsedSeconds :type "Float (double-precision)") (TriggeredSeconds :type "Float (double-precision)") (InputAction :type "InputAction Object Reference" :default "/Game/Game/GameMain/Input/IA_Decision.IA_Decision"))
  (:`Triggered`
    (set `self.PushButton` true)))

(fn `Play`
  (returns (isTaskEnd :type Boolean))
  (bind _dice (`self.Dice`))
  (bind _pushbutton (`self.PushButton`))
  (`/Game/Game/GameMain/SugorokuSystem/Dice/BP_SugorokuDice.StartRoll` _dice)
  (if _pushbutton
    (`/Game/Game/GameMain/SugorokuSystem/Dice/BP_SugorokuDice.StopRoll` _dice)
    (`self.K2_DestroyActor` (`self.Dice`))
    (return _pushbutton)))

(fn `UserConstructionScript`
  (`parent.UserConstructionScript`))