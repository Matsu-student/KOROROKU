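; BP_TileEffectTask is a game-loop task for the sugoroku board game's tile-effect step, though it applies no effect yet.
; Play searches all BP_PieceBase actors for the one whose PlayerID matches NowPlayerID and caches that piece's NowTile.
; It then prints a "TaskEffect" debug string and returns true immediately, without using the cached tile.
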(fn `Play`
  (returns (isTaskEnd :type Boolean))
  (bind _outactors (`GameplayStatics.GetAllActorsOfClass` "/Game/Game/GameMain/SugorokuSystem/Props/Pieces/BP_PieceBase.BP_PieceBase_C"))
  (for _array_element _outactors
    (if (== (`/Game/Game/GameMain/SugorokuSystem/Props/Pieces/BP_PieceBase.PlayerID` _array_element) (`self.NowPlayerID`))
      (set `self.Now Tile` (`/Game/Game/GameMain/SugorokuSystem/Props/Pieces/BP_PieceBase.NowTile` _array_element))
      (break)))
  (`KismetSystemLibrary.PrintString` "TaskEffect" true true (struct :`G` 0.66 :`B` 1.0 :`A` 1.0) 2.0 (`self.Key`))
  (return true))

(fn `UserConstructionScript`
  (`parent.UserConstructionScript`))