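; Base Blueprint for tasks in the sugoroku board game's game loop, holding the current player ID and a default Play that prints a debug message and returns true.
; Helpers include Wait, a call-counting frame delay, and Once, which returns false on first use and true afterward.
; InsertTask records a name, index, number and flag for a task to insert, which GetInsertTask exposes to callers.
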(event `/Game/Game/GameMain/SugorokuSystem/GameLoop/Tasks/Task/BI_Task.SetNowPlayerID`
  (params (PlayerID :type Name))
  (set `self.NowPlayerID` PlayerID))

(fn `GetInsertTask`
  (returns (TaskName :type Name) (Index :type Integer) (Number :type Integer) (IsInsertTask :type Boolean))
  (return (`self.InsertTaskName`) (`self.InsertIndex`) (`self.Number`) (`self.IsInsertTask`)))

(fn `Insert Task`
  (params (TaskName :type Name) (Index :type Integer) (Number :type Integer))
  (set `self.InsertTaskName` TaskName)
  (set `self.InsertIndex` Index)
  (set `self.Number` Number)
  (set `self.IsInsertTask` true)
  (return))

(fn `Once`
  (returns (IsUse :type Boolean))
  (locals (over :type Boolean :default false))
  (set `local.over` (> (`self.countUse`) 0))
  (`/Engine/EditorBlueprintResources/StandardMacros.IncrementInt` (`self.countUse`)
    (:`  `
      (return (`local.over`)))))

(fn `Play`
  (returns (isTaskEnd :type Boolean))
  (`KismetSystemLibrary.PrintString` (`KismetStringLibrary.Concat_StrStr` (`KismetStringLibrary.Conv_NameToString` (`self.Key`)) "/" "Play") true true (struct :`G` 0.66 :`B` 1.0 :`A` 1.0) 10.0 (`self.Key`))
  (return true))

(fn `UserConstructionScript`)

(fn `Wait`
  (params (Frame :type Integer))
  (returns (End :type Boolean))
  (bind _result (`/Engine/EditorBlueprintResources/StandardMacros.IncrementInt` (`self.CountFrame`))
    (:`  `
      (`KismetSystemLibrary.PrintString` (`KismetStringLibrary.Conv_IntToString` _result) true true (struct :`R` 1.0 :`B` 0.419177 :`A` 1.0) 2.0 "WaitTimer")
      (if (>= (`self.CountFrame`) Frame)
        (set `self.CountFrame` 0)
        (return true)
        (else
          (return false))))))