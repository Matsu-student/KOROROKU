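; BP_MovePicec is a game-loop task in the Sugoroku board game system that moves the game piece.
; On BeginPlay it caches the BP_PieceBase actor found through GetActorOfClass, so it works with a single piece.
; Its Play function calls InitMove and then Move on that piece, returning Move's result to the caller.
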(event `self.ReceiveBeginPlay`
  (`parent.ReceiveBeginPlay`)
  (bind _returnvalue (`GameplayStatics.GetActorOfClass` "/Game/Game/GameMain/SugorokuSystem/Props/Pieces/BP_PieceBase.BP_PieceBase_C"))
  (set `self.Piece` _returnvalue))

(fn `Play`
  (returns (isTaskEnd :type Boolean))
  (`/Game/Game/GameMain/SugorokuSystem/Props/Pieces/BP_PieceBase.InitMove` (`self.Piece`))
  (bind _end (`/Game/Game/GameMain/SugorokuSystem/Props/Pieces/BP_PieceBase.Move` (`self.Piece`)))
  (return _end))

(fn `UserConstructionScript`
  (`parent.UserConstructionScript`))