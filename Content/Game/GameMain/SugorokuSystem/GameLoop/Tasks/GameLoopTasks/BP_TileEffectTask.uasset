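; Sugoroku game-loop task that resolves the effects of the tile under the current player's piece.
; TaskInit finds the piece matching NowPlayerID and caches its tile's TileEffect and AddEffect.
; TaskPlay runs both through BP_TileEffectPlayer and inserts a requested follow-up task into the loop.
; When both request one, it sets MoreUseTask and returns false, inserting only the AddEffect task on the next call.
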(event `self.ReceiveBeginPlay`
  (`parent.ReceiveBeginPlay`)
  (bind _returnvalue (`GameplayStatics.GetActorOfClass` "/Game/Game/GameMain/SugorokuSystem/GameLoop/TileEffectPlayer/BP_TileEffectPlayer.BP_TileEffectPlayer_C"))
  (set `self.TileEffectPlayer` _returnvalue))

(event `/Game/Game/GameMain/SugorokuSystem/GameLoop/Tasks/Task/BI_Task.TaskInit`
  (`parent.TaskInit`)
  (bind _outactors (`GameplayStatics.GetAllActorsOfClass` "/Game/Game/GameMain/SugorokuSystem/Props/Pieces/BP_PieceBase.BP_PieceBase_C"))
  (for _array_element _outactors
    (if (== (`/Game/Game/GameMain/SugorokuSystem/Props/Pieces/BP_PieceBase.PlayerID` _array_element) (`self.NowPlayerID`))
      (bind _nowtile (`/Game/Game/GameMain/SugorokuSystem/Props/Pieces/BP_PieceBase.NowTile` _array_element))
      (set `self.Tile Effect` (`/Game/Game/GameMain/SugorokuSystem/Props/Tiles/Tile/BP_TileBase.TileEffect` _nowtile))
      (set `self.Add Effect` (`/Game/Game/GameMain/SugorokuSystem/Props/Tiles/Tile/BP_TileBase.AddEffect` _nowtile))
      (break))))

(fn `GetInsertTask`
  (returns (TaskName :type Name) (Index :type Integer) (Number :type Integer) (IsInsertTask :type Boolean))
  (bind (_taskname _index _number _isinserttask) (`parent.GetInsertTask`))
  (return _taskname _index _number _isinserttask))

(fn `Insert Task`
  (params (TaskName :type Name) (Index :type Integer) (Number :type Integer))
  (`parent.Insert Task` TaskName Index Number))

(fn `Once`
  (returns (IsUse :type Boolean))
  (bind _isuse (`parent.Once`))
  (return _isuse))

(fn `TaskPlay`
  (returns (isTaskEnd :type Boolean))
  (if (`self.MoreUseTask`)
    (`self.Insert Task` (stale _taskname_2) 1 1)
    (else
      (bind (_usenewtask _taskname) (`/Game/Game/GameMain/SugorokuSystem/GameLoop/TileEffectPlayer/BP_TileEffectPlayer.EffectPlay` (`self.TileEffectPlayer`) (`self.Tile Effect`)))
      (if _usenewtask
        (bind (_usenewtask_2 _taskname_2) (`/Game/Game/GameMain/SugorokuSystem/GameLoop/TileEffectPlayer/BP_TileEffectPlayer.EffectPlay` (`self.TileEffectPlayer`) (`self.Add Effect`)))
        (if _usenewtask_2
          (set `self.MoreUseTask` true)
          (return false)
          (else
            (`self.Insert Task` _taskname 0 1)))
        (else
          (bind (_usenewtask_3 _taskname_3) (`/Game/Game/GameMain/SugorokuSystem/GameLoop/TileEffectPlayer/BP_TileEffectPlayer.EffectPlay` (`self.TileEffectPlayer`) (`self.Add Effect`)))
          (if _usenewtask_3
            (`self.Insert Task` _taskname_3 0 1))))))
  (return true))

(fn `UserConstructionScript`
  (`parent.UserConstructionScript`))