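; AC_PlayerSwitcher tracks whose turn it is among four players in the sugoroku (board game) system.
; Switch increments an unwrapped Counter, indexes the PlayerID array by Counter modulo 4, prints a debug string, and returns the current ID and player number.
; GetNowPlayerID indexes the same array with the raw Counter, without the modulo wrap.
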(fn `GetNowPlayerID`
  (returns (NowPlayerID :type Name))
  (return (`|GetArrayItem` (`self.PlayerID`) (`self.Counter`))))

(fn `Switch`
  (returns (NowPlayerID :type Name) (PlayerNum :type Integer))
  (bind _returnvalue (mod (`self.Counter`) 4))
  (bind _output (`|GetArrayItem` (`self.PlayerID`) _returnvalue))
  (`/Engine/EditorBlueprintResources/StandardMacros.IncrementInt` (`self.Counter`)
    (:`  `
      (`KismetSystemLibrary.PrintString` (`KismetStringLibrary.Concat_StrStr` (`KismetStringLibrary.Conv_NameToString` (`self.Key`)) "/" (`KismetStringLibrary.Conv_NameToString` _output)) true true (struct :`G` 0.66 :`B` 1.0 :`A` 1.0) 2.0 (`self.Key`))
      (return _output _returnvalue))))