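; Task player component for the sugoroku system that runs queued named tasks one at a time.
; Process merges added names into the queue, spawns the first one's actor class via DT_TaskRegistration, and calls PlayMessage each call until it returns true.
; The finished actor is destroyed, and Process reports whether it was BP_EndTask.
; Del records removals, but the removal pass reads AddTask instead of DelTask, so they never apply.
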(fn `Add`
  (params (NewTask :type "Name (by ref)"))
  (`KismetArrayLibrary.Array_Add` (`self.AddTask`) NewTask))

(fn `ClassSerch`
  (params (Task :type Name))
  (returns (TaskClass :type "/Game/Game/GameMain/SugorokuSystem/Task/BP_TaskBase Class Reference"))
  (bind _outrownames (`DataTableFunctionLibrary.GetDataTableRowNames` "/Game/Game/GameMain/SugorokuSystem/Tasks/ClassRegistration/DT_TaskRegistration.DT_TaskRegistration"))
  (for _array_element _outrownames
    (bind _returnvalue (`|GetDataTableRow` "/Game/Game/GameMain/SugorokuSystem/Tasks/ClassRegistration/DT_TaskRegistration.DT_TaskRegistration" _array_element)
      (:`then`
        (bind (_taskname _taskclass) (break `/Game/Game/GameMain/SugorokuSystem/Tasks/ClassRegistration/F_TaskSearchData` _returnvalue))
        (if (== Task _taskname)
          (return _taskclass))))))

(fn `Del`
  (params (Task :type "Name (by ref)"))
  (`KismetArrayLibrary.Array_Add` (`self.DelTask`) Task))

(fn `Process`
  (returns (isEndPlay :type Boolean))
  (bind _addtask (`self.AddTask`))
  (bind _addtask_2 (`self.AddTask`))
  (if (> (`KismetArrayLibrary.Array_Length` (`self.AddTask`)) 0)
    (for _array_element _addtask_2
      (`KismetArrayLibrary.Array_Add` (`self.Tasks`) _array_element))
    (`KismetArrayLibrary.Array_Clear` _addtask_2))
  (if (`self.isPlay`) :!label _label
    (bind _istaskend (message `/Game/Game/GameMain/SugorokuSystem/Task/BI_Task.Play` (`self.Task`)))
    (if _istaskend
      (if (== (`GameplayStatics.GetObjectClass` (`self.Task`)) "/Game/Game/GameMain/SugorokuSystem/Tasks/BP_EndTask.BP_EndTask_C")
        (set `self.isEndPlay` true)
        (else
          (set `self.isEndPlay` false)))
      (`Actor.K2_DestroyActor` (`self.Task`))
      (set `self.isPlay` false)
      (if (> (`KismetArrayLibrary.Array_Length` (`self.DelTask`)) 0)
        (for _array_element_2 _addtask
          (for (_array_element_3 _array_index) (`self.Tasks`)
            (if (== _array_element_3 _array_element_2)
              (`KismetArrayLibrary.Array_Remove` (`self.Tasks`) _array_index)
              (break))))
        (`KismetArrayLibrary.Array_Clear` _addtask))
      (return (`self.isEndPlay`)))
    (else
      (bind _output_get (set `self.ProcessTask` (`|GetArrayItem` (`self.Tasks`)))) ; タスク名からタスク割り出し処理を書く
      (bind _taskclass (`self.ClassSerch` _output_get))
      (bind _returnvalue (`|SpawnActorFromClass` _taskclass (`KismetMathLibrary.MakeTransform` (0.0 0.0 0.0)) "Undefined" "MultiplyWithRoot" null null))
      (set `self.Task` _returnvalue)
      (if (> (`KismetArrayLibrary.Array_Length` (`self.Tasks`)) 0)
        (`KismetArrayLibrary.Array_Remove` (`self.Tasks`)))
      (set `self.isPlay` true)
      (goto _label))))