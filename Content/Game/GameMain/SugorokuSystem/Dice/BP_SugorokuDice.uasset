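; BP_SugorokuDice is a dice actor for the sugoroku board-game system, pairing a spinning cube with a number widget.
; Each StartRoll call hides the widget, writes a random number to it, and yaws the cube at a speed that climbs to a cap.
; StopRoll resets the cube and speed, then reveals the last number.
; The random range has MinNumber and MaxNumber wired to opposite inputs.
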(event `self.ReceiveBeginPlay`
  (bind _aswbp_sugoroku_dice (cast `/Game/Game/GameMain/SugorokuSystem/Dice/WBP_SugorokuDice` (`WidgetComponent.GetUserWidgetObject` (`self.Widget`))))
  (set `self.WBP Sugoroku Dice` _aswbp_sugoroku_dice))

(event `/Game/Game/GameMain/SugorokuSystem/Dice/BI_SugorokuDice.StartRoll`
  (`SceneComponent.SetVisibility` (`self.Widget`) false false)
  (bind _results (`self.Results`))
  (`/Game/Game/GameMain/SugorokuSystem/Dice/WBP_SugorokuDice.SetNumber` (`self.WBP Sugoroku Dice`) _results)
  (if (< (`self.RollSpeed`) (`self.MaxRollSpeed`))
    (bind _output_get (set `self.RollSpeed` (+ 1.0 (`self.RollSpeed`)))))
  (`SceneComponent.K2_AddRelativeRotation` (`self.Cube`) (`KismetMathLibrary.MakeRotator` 0.0 0.0 _output_get) false false))

(event `/Game/Game/GameMain/SugorokuSystem/Dice/BI_SugorokuDice.StopRoll`
  (`SceneComponent.K2_SetWorldRotation` :`self` (`self.Cube`))
  (set `self.RollSpeed` 0.0)
  (`SceneComponent.SetVisibility` (`self.Widget`) true false))

(fn `Results`
  (returns (Results :type Integer))
  (return (`KismetMathLibrary.RandomIntegerInRange` (`self.MaxNumber`) (`self.MinNumber`))))

(fn `UserConstructionScript`)