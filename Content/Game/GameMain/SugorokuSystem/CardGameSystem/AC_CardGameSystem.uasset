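; Card game component for the sugoroku board game that manages each player's card deck and hand slot.
; On BeginPlay it spawns a deck per player, links the card slot widgets and caches card data tables by type.
; Order events queue draw, display and selection-reset requests, which Process runs for the given player before flagging completion.
; SerchCardEffect turns a card's type and index into a task inserted through TaskPlayer.
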(event `self.ReceiveBeginPlay`
  ;[1 1 1] 人数分のカードデッキを作成
  (bind _outactors (`GameplayStatics.GetAllActorsOfClass` "/Game/Game/GameMain/SugorokuSystem/Player/BP_SugorokuPlayer.BP_SugorokuPlayer_C"))
  (for _array_element _outactors
    (bind _returnvalue (`|SpawnActorFromClass` "/Game/Game/GameMain/SugorokuSystem/CardGameSystem/Card/CardDeck/BP_CardDeck.BP_CardDeck_C" (`KismetMathLibrary.MakeTransform` (0.0 0.0 0.0)) "Undefined" "MultiplyWithRoot" null null))
    (`KismetArrayLibrary.Array_Add` (`self.CardDecks`) _returnvalue)
    (set `/Game/Game/GameMain/SugorokuSystem/CardGameSystem/Card/CardDeck/BP_CardDeckBase.PlayerID` (`/Game/Game/GameMain/SugorokuSystem/Player/BP_SugorokuPlayer.PlayerNum` _array_element) _returnvalue) ; PlayerIDをセット
  )
  ;[1 1 1] カードスロットを作成して保管
  (bind _foundwidgets (`WidgetBlueprintLibrary.GetAllWidgetsOfClass` "/Game/Game/GameMain/SugorokuSystem/CardGameSystem/Card/CardSlot/WBP_CardSlot.WBP_CardSlot_C" false))
  (bind _output_get (set `self.CardSlot` _foundwidgets))
  (for _array_element_2 _output_get
    (set `/Game/Game/GameMain/SugorokuSystem/CardGameSystem/Card/CardSlot/WBP_CardSlot.CardGameSystem` self _array_element_2))
  ;[1 1 1] カードデータを保管
  (for (_array_element_3 _array_index) (`self.CardDatas`)
    (bind _outrownames (`DataTableFunctionLibrary.GetDataTableRowNames` _array_element_3))
    (for _array_element_4 _outrownames
      (switch `int` _array_index
        (:`0`
          (bind _returnvalue_2 (`|GetDataTableRow` _array_element_3 _array_element_4)
            (:`then`
              (`KismetArrayLibrary.Array_Add` (`self.AttackCards`) _returnvalue_2))))
        (:`1`
          (bind _returnvalue_3 (`|GetDataTableRow` _array_element_3 _array_element_4)
            (:`then`
              (`KismetArrayLibrary.Array_Add` (`self.DefenceCards`) _returnvalue_3))))
        (:`2`
          (bind _returnvalue_4 (`|GetDataTableRow` _array_element_3 _array_element_4)
            (:`then`
              (`KismetArrayLibrary.Array_Add` (`self.RangeCards`) _returnvalue_4))))
        (:`3`
          (bind _returnvalue_5 (`|GetDataTableRow` _array_element_3 _array_element_4)
            (:`then`
              (`KismetArrayLibrary.Array_Add` (`self.EffectCards`) _returnvalue_5))))))))

(event `/Game/Game/GameMain/SugorokuSystem/CardGameSystem/BI_CardGameSystem.OrderDrawCard`
  ;[1 1 1] 命令文
  (`KismetArrayLibrary.Array_Add` (`self.OrderNums`) 1)
  (set `self.UseDrawCard` true)
  (set `self.IsOrder` true))

(event `/Game/Game/GameMain/SugorokuSystem/CardGameSystem/BI_CardGameSystem.OrderViewCards`
  ;[1 1 1] 命令文
  (`KismetArrayLibrary.Array_Add` (`self.OrderNums`) 2)
  (set `self.UseViewCards` true)
  (set `self.IsOrder` true))

(event `/Game/Game/GameMain/SugorokuSystem/CardGameSystem/BI_CardGameSystem.OrderInitCardSelect`
  ;[1 1 1] 命令文
  (`KismetArrayLibrary.Array_Add` (`self.OrderNums`) 3)
  (set `self.UseInitCardSelect` true)
  (set `self.IsOrder` true))

(fn `GetIsEndOrder`
  (returns (IsEndOrder :type Boolean))
  (return (`self.IsEndOrder`)))

(fn `Process`
  (params (NowPlayerID :type Integer))
  (locals (PlayerID :type Integer))
  (set `local.PlayerID` NowPlayerID)
  (if (`self.IsEndOrder`)
    (set `self.IsEndOrder` false)
    (elif (`self.IsOrder`)
      (for _array_element (`self.OrderNums`)
        (switch `int` _array_element
          (:`1`
            ;[1 1 1] カードを引いてスロットに登録
            (if (`self.UseDrawCard`)
              (bind _carddeck (`self.SerchCardDeckOfPlayer` (`local.PlayerID`)))
              (bind _returnvalue (`/Game/Game/GameMain/SugorokuSystem/CardGameSystem/Card/CardDeck/BP_CardDeckBase.DrawCard` _carddeck))
              (bind _cardslot (`self.SerchCardSlotOfPlayer` (`local.PlayerID`)))
              (`/Game/Game/GameMain/SugorokuSystem/CardGameSystem/Card/CardSlot/WBP_CardSlot.AddCard` _cardslot _returnvalue)))
          (:`2`
            ;[1 1 1] スロット内のカードを並べて表示
            (if (`self.UseViewCards`)
              (bind _cardslot_2 (`self.SerchCardSlotOfPlayer` (`local.PlayerID`)))
              (`/Game/Game/GameMain/SugorokuSystem/CardGameSystem/Card/CardSlot/WBP_CardSlot.ViweCards` _cardslot_2)))
          (:`3`
            ;[1 1 1] カード選択の初期化
            (if (`self.UseInitCardSelect`)
              (bind _cardslot_3 (`self.SerchCardSlotOfPlayer` (`local.PlayerID`)))
              (set `/Game/Game/GameMain/SugorokuSystem/CardGameSystem/Card/CardSlot/WBP_CardSlot.SelectNum` 0 _cardslot_3)
              (`/Game/Game/GameMain/SugorokuSystem/CardGameSystem/Card/CardSlot/WBP_CardSlot.TargetCard` _cardslot_3)))))
      (`KismetArrayLibrary.Array_Clear` (`self.OrderNums`))
      (set `self.IsOrder` false)
      (set `self.IsEndOrder` true)
      (set `self.CanSetPlayerID` true)
      (set `self.UseDrawCard` false)
      (set `self.UseViewCards` false)
      (set `self.UseInitCardSelect` false))))

(fn `SerchCardDeckOfPlayer`
  (params (NowPlayerID :type "Integer (by ref)"))
  (returns (CardDeck :type "/Game/Game/GameMain/SugorokuSystem/CardGameSystem/Card/CardDeck/BP_CardDeckBase Object Reference"))
  (for _array_element (`self.CardDecks`)
    (if (== (`/Game/Game/GameMain/SugorokuSystem/CardGameSystem/Card/CardDeck/BP_CardDeckBase.PlayerID` _array_element) NowPlayerID)
      (return _array_element))))

(fn `SerchCardEffect`
  (params (CardType :type "/Game/Game/GameMain/SugorokuSystem/CardGameSystem/Card/Cards/CardBase/Data/E_CardType Enum" :default "NewEnumerator0") (CardEffect :type Integer))
  (bind (_effectnum _taskname _insertindex _tasknum) (break `/Game/Game/GameMain/SugorokuSystem/CardGameSystem/Card/Cards/Registration/F_AttackCardSerchData` (`|GetArrayItem` (`self.AttackCards`) CardEffect)))
  (bind (_effectnum_2 _taskname_2 _insertindex_2 _tasknum_2) (break `/Game/Game/GameMain/SugorokuSystem/CardGameSystem/Card/Cards/Registration/F_DefenceCardSerchData` (`|GetArrayItem` (`self.DefenceCards`) CardEffect)))
  (bind (_effectnum_3 _taskname_3 _insertindex_3 _tasknum_3) (break `/Game/Game/GameMain/SugorokuSystem/CardGameSystem/Card/Cards/Registration/F_RangeCardSerchData` (`|GetArrayItem` (`self.RangeCards`) CardEffect)))
  (bind (_effectnum_4 _taskname_4 _insertindex_4 _tasknum_4) (break `/Game/Game/GameMain/SugorokuSystem/CardGameSystem/Card/Cards/Registration/F_EffectCardSerchData` (`|GetArrayItem` (`self.EffectCards`) CardEffect)))
  ;[1 1 1] カードをデータを検索
  (switch `/Game/Game/GameMain/SugorokuSystem/CardGameSystem/Card/Cards/CardBase/Data/E_CardType` CardType
    (:`NewEnumerator0`
      (message `/Game/Game/GameMain/SugorokuSystem/GameLoop/Task/TaskPlayer/BI_TaskPlayer.OrderInsert` (`self.TaskPlayer`) _taskname _insertindex _tasknum))
    (:`NewEnumerator1`
      (message `/Game/Game/GameMain/SugorokuSystem/GameLoop/Task/TaskPlayer/BI_TaskPlayer.OrderInsert` (`self.TaskPlayer`) _taskname_2 _insertindex_2 _tasknum_2))
    (:`NewEnumerator2`
      (message `/Game/Game/GameMain/SugorokuSystem/GameLoop/Task/TaskPlayer/BI_TaskPlayer.OrderInsert` (`self.TaskPlayer`) _taskname_3 _insertindex_3 _tasknum_3))
    (:`NewEnumerator3`
      (message `/Game/Game/GameMain/SugorokuSystem/GameLoop/Task/TaskPlayer/BI_TaskPlayer.OrderInsert` (`self.TaskPlayer`) _taskname_4 _insertindex_4 _tasknum_4)))
  (return))

(fn `SerchCardSlotOfPlayer`
  (params (NowPlayerID :type "Integer (by ref)"))
  (returns (CardSlot :type "/Game/Game/GameMain/SugorokuSystem/CardGameSystem/Card/CardSlot/WBP_CardSlot Object Reference"))
  (for _array_element (`self.CardSlot`)
    (if (== (`/Game/Game/GameMain/SugorokuSystem/CardGameSystem/Card/CardSlot/WBP_CardSlot.PlayerID` _array_element) NowPlayerID)
      (return _array_element))))