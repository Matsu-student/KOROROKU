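; BP_StartTile is the start tile of the sugoroku board game, where pieces are registered at setup.
; SetPieceStartTile points each piece's current and next tile at itself and sets its height to its box half-extent.
; It then hardcodes the on-tile piece count to four, regardless of array size, and calls SetPieceLocation, which defers positioning to the parent class.
; BeginPlay, overlap and construction only forward to the parent.
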(event `self.ReceiveBeginPlay`
  (`parent.ReceiveBeginPlay`))

(event `self.ReceiveActorBeginOverlap`
  (params (OtherActor :type "Actor Object Reference"))
  (`parent.ReceiveActorBeginOverlap` OtherActor))

(fn `SetPieceLocation`
  (`parent.SetPieceLocation`))

(fn `SetPieceStartTile`
  (params (Pieces :type "Array of /Game/Game/GameMain/SugorokuSystem/Props/Pieces/BP_PieceBase Object Reference"))
  (for _array_element Pieces
    (set `/Game/Game/GameMain/SugorokuSystem/Props/Pieces/BP_PieceBase.NextTile` self _array_element)
    (set `/Game/Game/GameMain/SugorokuSystem/Props/Pieces/BP_PieceBase.NowTile` self _array_element)
    (bind (_returnvalue_x _returnvalue_y) (`KismetMathLibrary.BreakVector` (`self.K2_GetActorLocation` _array_element)))
    (bind (_returnvalue_x_2 _returnvalue_y_2 _returnvalue_z) (`KismetMathLibrary.BreakVector` (`BoxComponent.GetScaledBoxExtent` (`/Game/Game/GameMain/SugorokuSystem/Props/Pieces/BP_PieceBase.Box` _array_element))))
    (`self.K2_SetActorLocation` _array_element (`KismetMathLibrary.MakeVector` _returnvalue_x _returnvalue_y _returnvalue_z) false false))
  (set `self.OnPiece` 4)
  (`self.SetPieceLocation`))

(fn `UserConstructionScript`
  (`parent.UserConstructionScript`))