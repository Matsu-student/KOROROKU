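; BP_Dice is the dice prop for the sugoroku board game system, pairing a spinning cube with a widget that displays the rolled number.
; Each StartRoll call hides the widget and advances the cube's yaw, ramping speed toward a maximum.
; StopRoll picks a random integer within the configured range, shows it through WBP_Dice and resets the cube's rotation and speed.
; The result is independent of the cube's orientation.
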(event `self.ReceiveBeginPlay`
  (bind _aswbp_dice (cast `/Game/Game/GameMain/SugorokuSystem/Props/Dice/WBP_Dice` (`WidgetComponent.GetUserWidgetObject` (`self.Widget`))))
  (set `self.WBPDice` _aswbp_dice)
  (`SceneComponent.SetVisibility` (`self.Widget`) false false))

(fn `Result`
  (returns (Number :type Integer))
  (return (`KismetMathLibrary.RandomIntegerInRange` (`self.MinResult`) (`self.MaxResult`))))

(fn `Start Roll`
  (`SceneComponent.SetVisibility` (`self.Widget`) false false)
  (if (< (`self.Rollspeed`) (`self.MaxRollspeed`))
    (bind _output_get (set `self.Rollspeed` (+ (`self.Rollspeed`) 1.0))))
  (`SceneComponent.K2_AddRelativeRotation` (`self.Cube`) (`KismetMathLibrary.MakeRotator` 0.0 0.0 _output_get) false false))

(fn `StopRoll`
  (bind _number (`self.Result`))
  (`/Game/Game/GameMain/SugorokuSystem/Props/Dice/WBP_Dice.SetNum` (`self.WBPDice`) _number)
  (`SceneComponent.SetVisibility` (`self.Widget`) true false)
  (`SceneComponent.K2_SetRelativeRotation` :`self` (`self.Cube`))
  (set `self.Rollspeed` 0.0))

(fn `UserConstructionScript`)