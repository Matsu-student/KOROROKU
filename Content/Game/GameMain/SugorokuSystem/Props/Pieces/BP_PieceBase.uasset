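; Base Blueprint for a sugoroku board game piece that travels between tiles along spline roads.
; InitMove adopts the tile queued by SetNowTile and starts progress at the spline end matching the travel direction.
; Each Move call steps along the first next or previous link, reporting completion or a selectable-tile stop.
; Only forward movement adds the box's height offset; SetLoacationOnTile snaps the piece to its tile in XY.
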(event `/Game/Game/GameMain/SugorokuSystem/Props/Pieces/BI_Piece.SetNowTile`
  (params (Tile :type "/Game/Game/GameMain/SugorokuSystem/Props/Tiles/Tile/BP_TileBase Object Reference"))
  (set `self.NextTile` Tile))

(fn `InitMove`
  (if (`self.NowDirection`)
    (if (not (`self.isMove`))
      (set `self.count` 0.0)
      (set `self.isMove` true)
      (set `self.NowTile` (`self.NextTile`)))
    (return)
    (else
      (if (not (`self.isMove`))
        (set `self.count` 1.0)
        (set `self.isMove` true)
        (set `self.NowTile` (`self.NextTile`)))
      (return))))

(fn `Move`
  (returns (End :type Boolean) (CanSelect :type Boolean))
  (bind (_returnvalue_x _returnvalue_y _returnvalue_z) (`KismetMathLibrary.BreakVector` (`BoxComponent.GetScaledBoxExtent` (`self.Box`))))
  (bind _spline (`/Game/Game/GameMain/SugorokuSystem/Props/Load/BP_LoadBase.Spline` (`self.Load`)))
  (bind _canselect (`/Game/Game/GameMain/SugorokuSystem/Props/Tiles/Tile/BP_TileBase.CanSelect` (`self.NowTile`)))
  (bind _spline_2 (`/Game/Game/GameMain/SugorokuSystem/Props/Load/BP_LoadBase.Spline` (`self.Load`)))
  (bind (_returnvalue_x_2 _returnvalue_y_2 _returnvalue_z_2) (`KismetMathLibrary.BreakVector` (`SplineComponent.GetLocationAtDistanceAlongSpline` _spline (* (`SplineComponent.GetSplineLength` _spline) (`self.count`)) "World")))
  (if _canselect
    (return true _canselect)
    (elif (`self.NowDirection`)
      (set `self.Load` (`|GetArrayItem` (`/Game/Game/GameMain/SugorokuSystem/Props/Tiles/Tile/BP_TileBase.NextTile` (`self.NowTile`))))
      (if (> (`self.count`) 1.0)
        (set `self.isMove` false)
        (return true false)
        (else
          (`self.K2_SetActorLocation` (`KismetMathLibrary.MakeVector` _returnvalue_x_2 _returnvalue_y_2 (+ _returnvalue_z_2 _returnvalue_z)))
          (set `self.count` (+ (`self.count`) (`self.MoveSpeed`)))
          (return false false)))
      (else
        (set `self.Load` (`|GetArrayItem` (`/Game/Game/GameMain/SugorokuSystem/Props/Tiles/Tile/BP_TileBase.BeforeTile` (`self.NowTile`))))
        (if (< (`self.count`) 0.0)
          (set `self.isMove` false)
          (return true false)
          (else
            (`self.K2_SetActorLocation` (`SplineComponent.GetLocationAtDistanceAlongSpline` _spline_2 (* (`SplineComponent.GetSplineLength` _spline_2) (`self.count`)) "World"))
            (set `self.count` (- (`self.count`) (`self.MoveSpeed`)))
            (return false false)))))))

(fn `SetLoacationOnTile`
  (bind (_returnvalue_x _returnvalue_y _returnvalue_z) (`KismetMathLibrary.BreakVector` (`self.K2_GetActorLocation`)))
  (bind (_returnvalue_x_2 _returnvalue_y_2) (`KismetMathLibrary.BreakVector` (`self.K2_GetActorLocation` (`self.NowTile`))))
  (`self.K2_SetActorLocation` (`KismetMathLibrary.MakeVector` _returnvalue_x_2 _returnvalue_y_2 _returnvalue_z)))

(fn `UserConstructionScript`)