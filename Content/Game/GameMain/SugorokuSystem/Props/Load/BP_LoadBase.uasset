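; Base road-style prop for the Sugoroku (board game) system that lays a flat mesh path along an editable spline.
; The construction script snaps the spline to the root's transform, then adds one spline mesh component per segment using the engine plane shape.
; Each piece takes its segment's local endpoints and tangents to follow the curve, with query and physics collision enabled.
; It has no runtime logic.
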(fn `UserConstructionScript`
  (bind _spline (`self.Spline`))
  (`SceneComponent.K2_SetWorldTransform` (`self.Spline`) (`SceneComponent.K2_GetComponentToWorld` (`self.DefaultSceneRoot`)) false false)
  (for _index (range (`SplineComponent.GetNumberOfSplineSegments` (`self.Spline`)))
    (bind _returnvalue (`AddComponent|NODE_AddSplineMeshComponent-0`))
    (`SceneComponent.K2_AttachToComponent` _returnvalue (`self.Spline`) "None" "KeepRelative" "KeepRelative" "KeepRelative" true)
    (`SplineMeshComponent.SetForwardAxis` _returnvalue "X" true)
    (`StaticMeshComponent.SetStaticMesh` _returnvalue "/Game/StarterContent/Shapes/Shape_Plane.Shape_Plane")
    (bind (_location _tangent) (`SplineComponent.GetLocationAndTangentAtSplinePoint` _spline _index "Local"))
    (bind (_location_2 _tangent_2) (`SplineComponent.GetLocationAndTangentAtSplinePoint` _spline (+ _index 1) "Local"))
    (`SplineMeshComponent.SetStartAndEnd` _returnvalue _location _tangent _location_2 _tangent_2 true)
    (`PrimitiveComponent.SetCollisionEnabled` _returnvalue "QueryAndPhysics")))